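; BP_SaveGame is the save data container for a space game, storing ship state, money, wave progress and player settings.
; Paired Set and Return functions write and read each group: basic transform and health, shields, guns, shared money and weapons, magnet and thruster systems, game mode and settings.
; A ClearAll event loops through SaveSlots, deletes each existing save and prints debug messages.
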(event `ClearAll`
  (for _array_element (`self.SaveSlots`)
    (bind _returnvalue (`GameplayStatics.DoesSaveGameExist` _array_element))
    (if _returnvalue
      (bind _returnvalue_2 (`GameplayStatics.DeleteGameInSlot` _array_element))
      (if _returnvalue_2
        (`KismetSystemLibrary.PrintString` null _array_element))))
  (`KismetSystemLibrary.PrintString` null "All Files deleted"))

(fn `ReturnBasic`
  (returns (Location :type "Vector Structure") (Rotation :type "Rotator Structure") (HealthCurrent :type "Float (double-precision)") (HealthMax :type "Float (double-precision)"))
  (return (`self.PlayerLocation`) (`self.PlayerRotation`) (`self.ShipHealthCurrent`) (`self.ShipHealthMax`)))

(fn `ReturnGameMode`
  (returns (Active :type Boolean) (Time :type "Float (double-precision)") (Wave :type Integer) (`1` :type Integer) (`2` :type Integer) (`3` :type Integer) (`4` :type Integer) (IdleTime :type "Float (double-precision)"))
  (return (`self.bWaveActive`) (`self.WaveTime`) (`self.WaveCurrent`) (`self.T1Count`) (`self.T2Count`) (`self.T3Count`) (`self.T4Count`) (`self.Idle`)))

(fn `ReturnGuns`
  (returns (Fire1 :type "Float (double-precision)") (Fire2 :type "Float (double-precision)") (Power1 :type "Float (double-precision)") (Power2 :type "Float (double-precision)"))
  (return (`self.GunFireRate1`) (`self.GunFireRate2`) (`self.GunPower1`) (`self.GunPower2`)))

(fn `ReturnSettings`
  (returns (ControllerType :type Integer) (`ClassicTurn?` :type Boolean) (Master :type "Float (double-precision)") (Music :type "Float (double-precision)") (SFX :type "Float (double-precision)"))
  (return (`self.ControllerScheme`) (`self.bUseClassicControls`) (`self.MasterVolume`) (`self.MusicVolume`) (`self.SFXVolume`)))

(fn `ReturnShared`
  (returns (Money :type Integer) (Left :type "/Game/Spacey_BP/Player/BP_ShipGunParent Class Reference") (Right :type "/Game/Spacey_BP/Player/BP_ShipGunParent Class Reference"))
  (return (`self.Money`) (`self.PlayerGunLeft`) (`self.PlayerGunRight`)))

(fn `ReturnShields`
  (returns (Max :type "Float (double-precision)") (Current :type "Float (double-precision)") (Drain :type "Float (double-precision)") (Regen :type "Float (double-precision)") (BootUp :type "Float (double-precision)") (BootUpCurrent :type "Float (double-precision)"))
  (return (`self.ShipShieldsMax`) (`self.ShipShieldsCurrent`) (`self.ShieldDrainRate`) (`self.ShieldRegenRate`) (`self.ShieldBootUp`) (`self.BootUpCurrent`)))

(fn `ReturnSystems`
  (returns (MagCurrent :type "Float (double-precision)") (MagMax :type "Float (double-precision)") (ThrustCurrent :type "Float (double-precision)") (ThrustMax :type "Float (double-precision)"))
  (return (`self.MagnetCurrent`) (`self.MagnetMax`) (`self.ThrusterCurrent`) (`self.ThrusterMax`)))

(fn `SetBasic`
  (params (Location :type "Vector Structure") (Rotation :type "Rotator Structure") (HealthCurrent :type "Float (double-precision)") (HealthMax :type "Float (double-precision)"))
  (set `self.PlayerLocation` Location)
  (set `self.PlayerRotation` Rotation)
  (set `self.ShipHealthCurrent` HealthCurrent)
  (set `self.ShipHealthMax` HealthMax))

(fn `SetGameMode`
  (params (Active :type Boolean) (Time :type "Float (double-precision)") (Wave :type Integer) (`1` :type Integer) (`2` :type Integer) (`3` :type Integer) (`4` :type Integer) (IdleTime :type "Float (double-precision)"))
  (set `self.bWaveActive` Active)
  (set `self.WaveTime` Time)
  (set `self.WaveCurrent` Wave)
  (set `self.T1Count` `1`)
  (set `self.T2Count` `2`)
  (set `self.T3Count` `3`)
  (set `self.T4Count` `4`)
  (set `self.Idle` IdleTime))

(fn `SetGuns`
  (params (Fire1 :type "Float (double-precision)") (Fire2 :type "Float (double-precision)") (Power1 :type "Float (double-precision)") (Power2 :type "Float (double-precision)"))
  (set `self.GunFireRate1` Fire1)
  (set `self.GunFireRate2` Fire2)
  (set `self.GunPower1` Power1)
  (set `self.GunPower2` Power2))

(fn `SetSettings`
  (params (ControllerType :type Integer) (`ClassicTurn?` :type Boolean) (Master :type "Float (double-precision)") (Music :type "Float (double-precision)") (SFX :type "Float (double-precision)"))
  (set `self.ControllerScheme` ControllerType)
  (set `self.bUseClassicControls` `ClassicTurn?`)
  (set `self.MasterVolume` Master)
  (set `self.MusicVolume` Music)
  (set `self.SFXVolume` SFX))

(fn `SetShared`
  (params (Money :type Integer) (Gun1 :type "/Game/Spacey_BP/Player/BP_ShipGunParent Class Reference") (Gun2 :type "/Game/Spacey_BP/Player/BP_ShipGunParent Class Reference"))
  (set `self.Money` Money)
  (set `self.PlayerGunLeft` Gun1)
  (set `self.PlayerGunRight` Gun2))

(fn `SetShields`
  (params (Max :type "Float (double-precision)") (Current :type "Float (double-precision)") (Drain :type "Float (double-precision)") (Regen :type "Float (double-precision)") (BootUp :type "Float (double-precision)") (BootupCurrent :type "Float (double-precision)"))
  (set `self.ShipShieldsMax` Max)
  (set `self.ShipShieldsCurrent` Current)
  (set `self.ShieldDrainRate` Drain)
  (set `self.ShieldRegenRate` Regen)
  (set `self.ShieldBootUp` BootUp)
  (set `self.BootUpCurrent` BootupCurrent))

(fn `SetSystems`
  (params (MagCurrent :type "Float (double-precision)") (MagMax :type "Float (double-precision)") (ThrustCurrent :type "Float (double-precision)") (ThrustMax :type "Float (double-precision)"))
  (set `self.MagnetCurrent` MagCurrent)
  (set `self.MagnetMax` MagMax)
  (set `self.ThrusterCurrent` ThrustCurrent)
  (set `self.ThrusterMax` ThrustMax))