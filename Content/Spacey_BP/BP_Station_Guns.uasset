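; Gun station Blueprint that opens the gun menu when its LoadUI event fires.
; It gets the widget and pilot from SetUILoad, which is defined outside this graph.
; It seeds BP_Guns_Widget with the pilot's fire, power and money values, then adds it to the viewport.
; An unconnected branch using BP_Widget_Station_Guns, which also set left and right guns, never runs.
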(event `self.LoadUI`
  (params (Actor :type "Actor Object Reference"))
  (bind (_pilot _outwidget) (`self.SetUILoad` Actor))
  (bind _asbp_guns_widget (cast `/Game/Spacey_BP/UI/Ship_Interior/BP_Guns_Widget` _outwidget))
  (`WidgetGuns.SetGunBaseValues` _asbp_guns_widget (`/Game/Spacey_BP/Player/BP_Pilot.Fire1` _pilot) (`/Game/Spacey_BP/Player/BP_Pilot.Fire2` _pilot) (`/Game/Spacey_BP/Player/BP_Pilot.Power1` _pilot) (`/Game/Spacey_BP/Player/BP_Pilot.Power2` _pilot) (`/Game/Spacey_BP/Player/BP_Pilot.Money` _pilot))
  (`UserWidget.AddToViewport` _asbp_guns_widget 0)
  (set `self.Actor` null))

(fn `UserConstructionScript`
  (`parent.UserConstructionScript`))