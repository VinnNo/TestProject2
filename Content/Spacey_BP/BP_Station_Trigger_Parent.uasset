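; Parent trigger for stations that lets an overlapping BP_Pilot open a menu by pressing Accept.
; Box overlaps store the pilot, toggle the prompt widget and player input, and play a sound.
; Accept calls LoadUI, an empty hook for child Blueprints.
; The SetUILoad helper disables pilot movement, creates the UIWidget, and assigns it and MenuNumber to the pilot.
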(event `self.ReceiveBeginPlay`
  ;[1 1 1] Begin Play
  (`SceneComponent.SetVisibility` (`self.Widget`) false false)
  (set `self.bCanOverlap` true)
  (`self.DisableInput` (`GameplayStatics.GetPlayerController` 0)))

(event `self.Box.OnComponentBeginOverlap`
  (params (OverlappedComponent :type "PrimitiveComponent Object Reference") (OtherActor :type "Actor Object Reference") (OtherComp :type "PrimitiveComponent Object Reference") (OtherBodyIndex :type Integer) (bFromSweep :type Boolean) (SweepResult :type "HitResult Structure (by ref)"))
  ;[1 1 1] OverLaps
  (if (`self.bCanOverlap`)
    (bind _asbp_pilot (cast `/Game/Spacey_BP/Player/BP_Pilot` OtherActor))
    (set `self.Actor` _asbp_pilot)
    (set `/Game/Spacey_BP/Player/BP_Pilot.OverlappingStation` self _asbp_pilot)
    (`SceneComponent.SetVisibility` (`self.Widget`) true false)
    (`self.EnableInput` (`GameplayStatics.GetPlayerController` 0))
    (`GameplayStatics.PlaySoundAtLocation` "/Game/Spacey/Audio/SFX/Menus/Widets/maximize_006.maximize_006" (`self.K2_GetActorLocation`) (struct) 1.0 1.0 0.0 null null null)))

(event `self.Box.OnComponentEndOverlap`
  (params (OverlappedComponent :type "PrimitiveComponent Object Reference") (OtherActor :type "Actor Object Reference") (OtherComp :type "PrimitiveComponent Object Reference") (OtherBodyIndex :type Integer))
  ;[1 1 1] OverLaps
  (bind _asbp_pilot (cast `/Game/Spacey_BP/Player/BP_Pilot` OtherActor))
  (set `self.Actor` null)
  (set `/Game/Spacey_BP/Player/BP_Pilot.OverlappingStation` null _asbp_pilot)
  (`SceneComponent.SetVisibility` (`self.Widget`) false false)
  (`self.DisableInput` (`GameplayStatics.GetPlayerController` 0))
  (`GameplayStatics.PlaySoundAtLocation` "/Game/Spacey/Audio/SFX/Menus/Widets/minimize_006.minimize_006" (`self.K2_GetActorLocation`) (struct) 1.0 1.0 0.0 null null null))

(event `InputAction|Accept`
  (params (Key :type "Key Structure"))
  ;[1 1 1] Inputs
  (:`Pressed`
    (if (and (`KismetSystemLibrary.IsValid` (`self.Actor`)) (`SceneComponent.IsVisible` (`self.Widget`)))
      (`self.LoadUI` (`self.Actor`))
      (`self.DisableInput` (`GameplayStatics.GetPlayerController` 0)))))

(event `LoadUI`
  (params (Actor :type "Actor Object Reference"))
  ;[1 1 1] Dummy function for children
)

(fn `SetUILoad`
  (params (InActor :type "Actor Object Reference"))
  (returns (Pilot :type "/Game/Spacey_BP/Player/BP_Pilot Object Reference") (OutWidget :type "UserWidget Object Reference"))
  (locals (Widget :type "UserWidget Object Reference"))
  (bind _asbp_pilot (cast `/Game/Spacey_BP/Player/BP_Pilot` InActor))
  (`/Game/Spacey_BP/Player/BP_Pilot.SetMove` _asbp_pilot false)
  (bind _returnvalue (`|CreateWidget` (`self.UIWidget`) (`GameplayStatics.GetPlayerController` 0)))
  (bind _output_get (set `/Game/Spacey_BP/Player/BP_Pilot.CurrentMenu` _returnvalue _asbp_pilot))
  (set `/Game/Spacey_BP/Player/BP_Pilot.MenuNumber` (`self.MenuNumber`) _asbp_pilot)
  (return _asbp_pilot _output_get))

(fn `UserConstructionScript`)