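; BP_Station_Pilot is a station Blueprint that opens the pilot station's UI when its LoadUI event fires.
; LoadUI passes the given Actor to SetUILoad, then casts the returned widget to BP_Widget_Station_Pilot.
; It hands the widget the returned pilot as Player along with DisplayText, adds it to the viewport, then clears the Actor reference.
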(event `self.LoadUI`
  (params (Actor :type "Actor Object Reference"))
  (bind (_pilot _outwidget) (`self.SetUILoad` Actor))
  (bind _asbp_widget_station_pilot (cast `/Game/Spacey_BP/UI/Ship_Interior/BP_Widget_Station_Pilot` _outwidget))
  (set `/Game/Spacey_BP/UI/Ship_Interior/BP_Widget_Station_Pilot.Player` _pilot _asbp_widget_station_pilot)
  (set `/Game/Spacey_BP/UI/Ship_Interior/BP_Widget_Station_Pilot.DisplayText` (`self.DisplayText`) _asbp_widget_station_pilot)
  (`UserWidget.AddToViewport` _asbp_widget_station_pilot 0)
  (set `self.Actor` null))

(fn `UserConstructionScript`
  (`parent.UserConstructionScript`))