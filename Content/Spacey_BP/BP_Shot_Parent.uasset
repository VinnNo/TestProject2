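; BP_Shot_Parent is a projectile Blueprint, apparently the base for shots in a space game, that destroys itself once its Lifetime expires.
; DeathEvent stops the projectile movement, spawns DeathParticle at the shot's location, then destroys the actor after a short delay.
; Its IsNotPlayer input is unused, as the branch that would attach the particle to BP_PlayerShip's mesh is disconnected and never runs.
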(event `self.ReceiveBeginPlay`
  (`KismetSystemLibrary.Delay` (`self.Lifetime`))
  (`self.K2_DestroyActor`))

(event `DeathEvent`
  (params (`IsNotPlayer?` :type Boolean))
  (set `MovementComponent.Velocity` (0.0 0.0 0.0) (`self.ProjectileMovement`))
  (`GameplayStatics.SpawnEmitterAtLocation` (`self.DeathParticle`) (`self.K2_GetActorLocation`))
  (`KismetSystemLibrary.Delay` 0.2)
  (`self.K2_DestroyActor`))

(fn `UserConstructionScript`)