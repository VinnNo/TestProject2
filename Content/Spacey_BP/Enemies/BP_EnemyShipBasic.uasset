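; Basic AI enemy ship that patrols, pursues and shoots the player, then explodes and drops gems.
; A four-state machine (idle, move, move and fire, fire) drives AIMoveTo and child-actor guns, halting when the player dies.
; Sight overlaps with line-of-sight checks, shot damage and patrol timeouts change state.
; Health depletion triggers randomized explosion effects and loot, and the game mode tracks spawned and destroyed ships.
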(event `SightEntered`
  (params (`Other Actor` :type "Actor Object Reference") (OtherComponent :type "ActorComponent Object Reference"))
  (bind _asbp_player_ship (cast `/Game/Spacey_BP/Player/BP_PlayerShip` `Other Actor`))
  (if (== OtherComponent (`PlayerShipBase.ShipMeshComponent` _asbp_player_ship))
    (bind _returnvalue (`self.InLineOfSight` (`self.K2_GetActorLocation` _asbp_player_ship) true))
    (if _returnvalue
      (`self.SetState` 3))))

(event `SightLeft`
  (params (`Other Actor` :type "Actor Object Reference") (OtherComponent :type "ActorComponent Object Reference"))
  (bind _asbp_player_ship (cast `/Game/Spacey_BP/Player/BP_PlayerShip` `Other Actor`))
  (if (== OtherComponent (`PlayerShipBase.ShipMeshComponent` _asbp_player_ship))
    (bind _returnvalue (`self.InLineOfSight` (`self.K2_GetActorLocation` _asbp_player_ship)))
    (if _returnvalue
      (`self.SetState` 2))))

(event `self.Sight.OnComponentBeginOverlap`
  (params (OverlappedComponent :type "PrimitiveComponent Object Reference") (OtherActor :type "Actor Object Reference") (OtherComp :type "PrimitiveComponent Object Reference") (OtherBodyIndex :type Integer) (bFromSweep :type Boolean) (SweepResult :type "HitResult Structure (by ref)"))
  (bind _asbp_player_ship (cast `/Game/Spacey_BP/Player/BP_PlayerShip` OtherActor))
  (bind _returnvalue (`self.InLineOfSight` (`self.K2_GetActorLocation` _asbp_player_ship) true))
  (if _returnvalue
    (`self.SetState` 3)))

(event `TakeDamage`
  (params (OtherActor :type "Actor Object Reference"))
  (bind _asbp_shot_parent (cast `/Game/Spacey_BP/BP_Shot_Parent` OtherActor))
  (`HealthComponent.DecrementHealth` (`self.Health`) (`/Game/Spacey_BP/BP_Shot_Parent.Damage` _asbp_shot_parent))
  (`self.SetState` 2))

(event `self.Sight.OnComponentEndOverlap`
  (params (OverlappedComponent :type "PrimitiveComponent Object Reference") (OtherActor :type "Actor Object Reference") (OtherComp :type "PrimitiveComponent Object Reference") (OtherBodyIndex :type Integer))
  (bind _asbp_player_ship (cast `/Game/Spacey_BP/Player/BP_PlayerShip` OtherActor))
  (bind _returnvalue (`self.InLineOfSight` (`self.K2_GetActorLocation` _asbp_player_ship)))
  (if _returnvalue
    (`self.SetState` 2)))

(event `self.FoundPlayer`
  (if (or (== (`self.STATE`) 0) (== (`self.STATE`) 1))
    (`self.SetState` 2)))

(event `self.PatrolTimerUp`
  (bind _returnvalue (`self.InLineOfSight` (`self.TargetLocation`) true))
  (if (not _returnvalue)
    (`self.SetState` 0)
    (else
      (`self.SetState` 2))))

(event `self.ReceiveBeginPlay`
  (if (`self.bIsDebug`)
    (`SceneComponent.SetHiddenInGame` (`self.CapsuleComponent`) false false)
    (`SceneComponent.SetHiddenInGame` (`self.Sight`) false false)
    (else
      (`SceneComponent.SetHiddenInGame` (`self.CapsuleComponent`) true false)
      (`SceneComponent.SetHiddenInGame` (`self.Sight`) true false)))
  (`self.SetState` 0)
  (`KismetSystemLibrary.Delay` 0.01)
  (`self.SetState` 0)
  (add `self.OnGemSpawn` (delegate `OnGemSpawn_Event_0`))
  (bind _asbp_game_mode_ship (cast `/Game/Spacey_BP/BP_GameMode_Ship` (`GameplayStatics.GetGameMode`)))
  (`GameModeShip.UpdateEnemyShipCount` _asbp_game_mode_ship))

(event `self.OnStateChanged`
  (bind _state (`self.STATE`))
  (bind _asbp_game_mode_ship (cast `/Game/Spacey_BP/BP_GameMode_Ship` (`GameplayStatics.GetGameMode`)))
  (if (not (`GameModeShip.bPlayerDead` _asbp_game_mode_ship))
    (switch `int` (`self.STATE`)
      (:`0`
        (`self.SetFire` false)
        (`KismetSystemLibrary.RetriggerableDelay` (`self.IdleTime`))
        (`self.SetState` 1))
      (:`1`
        (`|AIMoveTo` self (`self.TargetLocation`) (`self.TargetActor`) (`self.Acceptance`)
          (:`then`
            (`self.SetFire` false))
          (:`OnSuccess`
            (`self.SetState` 1 :!label _label)
            (`KismetSystemLibrary.Delay` 0.2)
            (if (or (== _state 0) (== _state 1))
              (`self.SetState` 1)))
          (:`OnFail`
            (goto _label))))
      (:`2`
        (`|AIMoveTo` self (`self.TargetLocation`) (`self.TargetActor`) (`self.Acceptance`)
          (:`then`
            (`self.StartPatrolTimer` false)
            (`self.SetFire` true))))
      (:`3`
        (`self.SetFire` true)))
    (else
      (`self.SetState` 0)
      (`MovementComponent.StopMovementImmediately` (`self.CharacterMovement`)))))

(event `self.ShipMeshComponent.OnComponentBeginOverlap`
  (params (OverlappedComponent :type "PrimitiveComponent Object Reference") (OtherActor :type "Actor Object Reference") (OtherComp :type "PrimitiveComponent Object Reference") (OtherBodyIndex :type Integer) (bFromSweep :type Boolean) (SweepResult :type "HitResult Structure (by ref)"))
  (bind _asbp_shot_parent (cast `/Game/Spacey_BP/BP_Shot_Parent` OtherActor))
  (`HealthComponent.DecrementHealth` (`self.Health`) (`/Game/Spacey_BP/BP_Shot_Parent.Damage` _asbp_shot_parent))
  (`self.SetState` 2))

(event `OnGemSpawn_Event_0` :!signature `self.OnGemSpawn`
  (params (SpawnSize :type Integer))
  (switch `int` SpawnSize
    (:`1`
      (`|SpawnActorFromClass` "/Game/Spacey_BP/Pickups/BP_Gem_Low.BP_Gem_Low_C" (`KismetMathLibrary.MakeTransform` (+ (`self.K2_GetActorLocation`) (`self.RandomizeVector` (* (`self.DeathParticleRange`) (`self.LootSpawnMultiplier`))))) "Undefined" "OverrideRootScale" null null))
    (:`2`
      (`|SpawnActorFromClass` "/Game/Spacey_BP/Pickups/BP_Gem_Medium.BP_Gem_Medium_C" (`KismetMathLibrary.MakeTransform` (+ (`self.K2_GetActorLocation`) (`self.RandomizeVector` (* (`self.DeathParticleRange`) (`self.LootSpawnMultiplier`))))) "Undefined" "OverrideRootScale" null null))
    (:`3`
      (`|SpawnActorFromClass` "/Game/Spacey_BP/Pickups/BP_Gem_Large.BP_Gem_Large_C" (`KismetMathLibrary.MakeTransform` (+ (`self.K2_GetActorLocation`) (`self.RandomizeVector` (* (`self.DeathParticleRange`) (`self.LootSpawnMultiplier`))))) "Undefined" "OverrideRootScale" null null))))

(event `self.Health.OnHealthDepleted`
  (`self.Do Death`))

(fn `Do Death`
  (locals (RandomLoation :type "Vector Structure"))
  (for _ (range (+ (`self.DeathParticleCount`) 1))
    (bind _output_get (set `local.RandomLoation` (+ (`self.K2_GetActorLocation`) (`self.RandomizeVector` (`self.DeathParticleRange`)))))
    (`GameplayStatics.SpawnEmitterAtLocation` "/Game/Spacey/Particles/p_EnemyShotDeath.p_EnemyShotDeath" _output_get (struct) (3.0 3.0 3.0)))
  (bind _sound (`self.Randomized Explosion SFX`))
  (`GameplayStatics.PlaySoundAtLocation` _sound (`self.K2_GetActorLocation`) (struct) 1.0 1.0 0.0 null null null)
  (bind _bcomplete (`self.SpawnLoot`))
  (if _bcomplete
    (bind _asbp_game_mode_ship (cast `/Game/Spacey_BP/BP_GameMode_Ship` (`GameplayStatics.GetGameMode`)))
    (`/Engine/EditorBlueprintResources/StandardMacros.IsValid` _asbp_game_mode_ship
      (:`Is Valid`
        (`/Game/Spacey_BP/BP_GameMode_Ship.EnemyShipDeath` _asbp_game_mode_ship)
        (`self.K2_DestroyActor`)))))

(fn `Randomized Explosion SFX`
  (returns (Sound :type "SoundBase Object Reference"))
  (locals (SFX :type "SoundBase Object Reference"))
  (bind _returnvalue (`KismetMathLibrary.RandomFloatInRange` 1.0 100.0))
  (`|ExecutionSequence`
    (:`then_0`
      (if (< _returnvalue 20.0)
        (set `local.SFX` "/Game/Spacey/Audio/SFX/Explosions/explosionCrunch_000.explosionCrunch_000")
        (elif (< _returnvalue 40.0)
          (set `local.SFX` "/Game/Spacey/Audio/SFX/Explosions/explosionCrunch_001.explosionCrunch_001")
          (elif (< _returnvalue 60.0)
            (set `local.SFX` "/Game/Spacey/Audio/SFX/Explosions/explosionCrunch_002.explosionCrunch_002")
            (elif (< _returnvalue 80.0)
              (set `local.SFX` "/Game/Spacey/Audio/SFX/Explosions/explosionCrunch_003.explosionCrunch_003")
              (else
                (set `local.SFX` "/Game/Spacey/Audio/SFX/Explosions/explosionCrunch_004.explosionCrunch_004")))))))
    (:`then_1`
      (return (`local.SFX`)))))

(fn `RandomizeVector`
  (params (InVector :type "Vector Structure"))
  (returns (OutVector :type "Vector Structure"))
  (return (`KismetMathLibrary.MakeVector` (`KismetMathLibrary.RandomFloatInRange` (- 0.0 InVector_X) InVector_X) (`KismetMathLibrary.RandomFloatInRange` (- 0.0 InVector_Y) InVector_Y) (`KismetMathLibrary.RandomFloatInRange` (- 0.0 InVector_Z) InVector_Z))))

(fn `SetFire`
  (params (`Fire?` :type Boolean))
  (locals (Fire :type Boolean))
  (for _array_element (`self.GetAllChildActors` true)
    (bind _asbp_enemy_gun_1 (cast `/Game/Spacey_BP/Enemies/BP_EnemyGun1` _array_element))
    (if `Fire?`
      (set `/Game/Spacey_BP/Enemies/BP_EnemyGun1.Parent` self _asbp_enemy_gun_1)
      (`/Game/Spacey_BP/Enemies/BP_EnemyGun1.Shoot` _asbp_enemy_gun_1)
      (set `/Game/Spacey_BP/Enemies/BP_EnemyGun1.bLoop?` true _asbp_enemy_gun_1)
      (else
        (set `/Game/Spacey_BP/Enemies/BP_EnemyGun1.bLoop?` false _asbp_enemy_gun_1)))))

(fn `UserConstructionScript`)