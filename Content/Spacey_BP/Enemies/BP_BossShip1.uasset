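; Boss enemy ship that attacks the player with child guns and paired rocket launchers.
; A state machine randomly alternates between chasing with rockets, holding fire on target and a rapid-fire spin without rockets.
; Sight sphere overlaps with the player also switch states, except during a spin.
; Shot overlaps drain the Health component (the state reaction is disabled); depletion triggers explosions, gem loot and a game mode death notification.
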(event `self.ReceiveBeginPlay`
  (bind _returnvalue (`SphereComponent.GetUnscaledSphereRadius` (`self.Sight`)))
  (if (`self.bIsDebug`)
    (`SceneComponent.SetHiddenInGame` (`self.CapsuleComponent`) false false)
    (`SceneComponent.SetHiddenInGame` (`self.Sight`) false false)
    (else
      (`SceneComponent.SetHiddenInGame` (`self.CapsuleComponent`) true false)
      (`SceneComponent.SetHiddenInGame` (`self.Sight`) true false)))
  (`self.SetState` 2)
  (add `self.OnGemSpawn` (delegate `OnGemSpawn_Event_0`))
  (`KismetSystemLibrary.Delay` 0.01)
  (set `self.AcceptanceFound` _returnvalue)
  (set `self.AcceptanceLost` (/ _returnvalue 2.0))
  (bind _asbp_game_mode_ship (cast `/Game/Spacey_BP/BP_GameMode_Ship` (`GameplayStatics.GetGameMode`)))
  (`GameModeShip.UpdateEnemyShipCount` _asbp_game_mode_ship))

(event `self.OnStateChanged`
  (switch `int` (`self.STATE`)
    (:`0`
      (`NavMovementComponent.StopActiveMovement` (`self.CharacterMovement`))
      (`self.SetFireRates` true)
      (`self.SetFire` true)
      (`|ExecutionSequence`
        (:`then_0`
          (if (> (`KismetMathLibrary.RandomFloatInRange` -10.0 10.0) 0.0)
            (set `self.RotDir` 1.0)
            (else
              (set `self.RotDir` -1.0)))
          (set `RotatingMovementComponent.RotationRate` (`KismetMathLibrary.MakeRotator` 0.0 0.0 (* (`self.RotSpeed`) (`self.RotDir`))) (`self.RotatingMovement1`))
          (set `self.bShouldRotate` false)
          (`self.SetRocketFire` false))
        (:`then_1`
          (`KismetSystemLibrary.Delay` (`self.SpinTime`))
          (`self.SetState` 2)
          (set `RotatingMovementComponent.RotationRate` (struct) (`self.RotatingMovement1`))
          (set `self.bShouldRotate` true))))
    (:`1`
      (`self.SetFireRates` false)
      (`self.SetFire` true)
      (`self.SetRocketFire` false))
    (:`2`
      (`|AIMoveTo` self (`self.TargetLocation`) (`self.TargetActor`) (`self.Acceptance`)
        (:`then`
          (`self.SetFire` true)
          (`self.SetFireRates` false)
          (`self.SetRocketFire` true))
        (:`OnSuccess`
          (if (> (`KismetMathLibrary.RandomFloatInRange` 1.0 100.0) 80.0)
            (`self.SetState` 0)
            (else
              (`self.SetState` 3))))))
    (:`3`
      (`self.SetFire` true)
      (`self.SetFireRates` false)
      (`self.SetRocketFire` true)
      (`KismetSystemLibrary.Delay` 5.0)
      (if (and (!= (`self.STATE`) 0) (> (`KismetMathLibrary.RandomFloatInRange` 1.0 100.0) 50.0))
        (`self.SetState` 0)
        (else
          (`self.SetState` 2))))
    (:`4`
      (`self.SetFire` false)
      (`self.SetFireRates` false)
      (`self.SetRocketFire` false))))

(event `OnGemSpawn_Event_0`
  (params (SpawnSize :type Integer))
  (switch `int` SpawnSize
    (:`1`
      (`|SpawnActorFromClass` "/Game/Spacey_BP/Pickups/BP_Gem_Low.BP_Gem_Low_C" (`KismetMathLibrary.MakeTransform` (+ (`self.K2_GetActorLocation`) (`StaticsLibrary.RandomizeVector` (* (`self.DeathParticleRange`) (`self.LootSpawnMultiplier`))))) "Undefined" "OverrideRootScale" null null))
    (:`2`
      (`|SpawnActorFromClass` "/Game/Spacey_BP/Pickups/BP_Gem_Medium.BP_Gem_Medium_C" (`KismetMathLibrary.MakeTransform` (+ (`self.K2_GetActorLocation`) (`StaticsLibrary.RandomizeVector` (* (`self.DeathParticleRange`) (`self.LootSpawnMultiplier`))))) "Undefined" "OverrideRootScale" null null))
    (:`3`
      (`|SpawnActorFromClass` "/Game/Spacey_BP/Pickups/BP_Gem_Large.BP_Gem_Large_C" (`KismetMathLibrary.MakeTransform` (+ (`self.K2_GetActorLocation`) (`StaticsLibrary.RandomizeVector` (* (`self.DeathParticleRange`) (`self.LootSpawnMultiplier`))))) "Undefined" "OverrideRootScale" null null))))

(event `self.Sight.OnComponentBeginOverlap`
  (params (OverlappedComponent :type "PrimitiveComponent Object Reference") (OtherActor :type "Actor Object Reference") (OtherComp :type "PrimitiveComponent Object Reference") (OtherBodyIndex :type Integer) (bFromSweep :type Boolean) (SweepResult :type "HitResult Structure (by ref)"))
  (bind _asbp_player_ship (cast `/Game/Spacey_BP/Player/BP_PlayerShip` OtherActor))
  (if (and (== (`Actor.RootComponent` _asbp_player_ship) OtherComp) (!= (`self.STATE`) 0))
    (if (> (`KismetMathLibrary.RandomFloatInRange` 1.0 100.0) 40.0)
      (`self.SetState` 3)
      (else
        (`self.SetState` 0)))))

(event `self.Sight.OnComponentEndOverlap`
  (params (OverlappedComponent :type "PrimitiveComponent Object Reference") (OtherActor :type "Actor Object Reference") (OtherComp :type "PrimitiveComponent Object Reference") (OtherBodyIndex :type Integer))
  (bind _asbp_player_ship (cast `/Game/Spacey_BP/Player/BP_PlayerShip` OtherActor))
  (if (and (== (`Actor.RootComponent` _asbp_player_ship) OtherComp) (!= (`self.STATE`) 0))
    (`self.SetState` 2)))

(event `self.ShipMeshComponent.OnComponentBeginOverlap`
  (params (OverlappedComponent :type "PrimitiveComponent Object Reference") (OtherActor :type "Actor Object Reference") (OtherComp :type "PrimitiveComponent Object Reference") (OtherBodyIndex :type Integer) (bFromSweep :type Boolean) (SweepResult :type "HitResult Structure (by ref)"))
  (bind _health (`self.Health`))
  (bind _asbp_shot_parent (cast `/Game/Spacey_BP/BP_Shot_Parent` OtherActor))
  (`HealthComponent.DecrementHealth` (`self.Health`) (`/Game/Spacey_BP/BP_Shot_Parent.Damage` _asbp_shot_parent))
  (if (and (!= (`self.STATE`) 0) false)
    (`/Engine/EditorBlueprintResources/StandardMacros.IsValid` _health
      (:`Is Valid`
        (if (> (`KismetMathLibrary.Vector_Distance` (`self.K2_GetActorLocation` (`GameplayStatics.GetPlayerPawn` 0)) (`self.K2_GetActorLocation`)) 3000.0)
          (`self.SetState` 2)
          (elif (< (`HealthComponent.GetHealthAsPercent` _health) 0.5)
            (`self.SetState` 0)))))))

(event `self.Health.OnHealthDepleted`
  (`self.DoDeath`))

(event `SetRocketFire`
  (params (`SetFire?` :type Boolean))
  (bind _output_get (set `self.RocketShoot` `SetFire?`))
  (if _output_get
    (`self.FireRockets` true)))

(event `FireRockets`
  (params (fire :type Boolean))
  (if (and fire (`self.bCanFireFocket`))
    (`|ExecutionSequence`
      (:`then_0`
        (`|SpawnActorFromClass` "/Game/Spacey_BP/Enemies/BP_BossShot1.BP_BossShot1_C" (`SceneComponent.K2_GetComponentToWorld` (`self.RocketArrowRight`)) "Undefined" "OverrideRootScale" null null))
      (:`then_1`
        (`|SpawnActorFromClass` "/Game/Spacey_BP/Enemies/BP_BossShot1.BP_BossShot1_C" (`SceneComponent.K2_GetComponentToWorld` (`self.RocketArrowLeft`)) "Undefined" "OverrideRootScale" null null))
      (:`then_2`
        (set `self.bCanFireFocket` false)
        (`KismetSystemLibrary.RetriggerableDelay` (`self.RocketFireRate`))
        (set `self.bCanFireFocket` true)
        (if (`self.RocketShoot`)
          (`self.FireRockets` true))))))

(fn `DoDeath`
  (locals (RandomLocation :type "Vector Structure"))
  (for _ (range 21)
    (bind _output_get (set `local.RandomLocation` (+ (`self.K2_GetActorLocation`) (`StaticsLibrary.RandomizeVector` (`self.DeathParticleRange`)))))
    (`GameplayStatics.SpawnEmitterAtLocation` "/Game/Spacey/Particles/p_EnemyShotDeath.p_EnemyShotDeath" _output_get (struct) (3.0 3.0 3.0)))
  (bind _bcomplete (`self.SpawnLoot`))
  (if _bcomplete
    (bind _asbp_game_mode_ship (cast `/Game/Spacey_BP/BP_GameMode_Ship` (`GameplayStatics.GetGameMode`))
      (:`then`
        (`/Engine/EditorBlueprintResources/StandardMacros.IsValid` _asbp_game_mode_ship
          (:`Is Valid`
            (`/Game/Spacey_BP/BP_GameMode_Ship.EnemyShipDeath` _asbp_game_mode_ship))))
      (:`CastFailed`
        _))
    (`self.K2_DestroyActor`)))

(fn `SetFire`
  (params (Fire :type Boolean))
  (for _array_element (`self.GetAllChildActors` true)
    (bind _asbp_enemy_gun_1 (cast `/Game/Spacey_BP/Enemies/BP_EnemyGun1` _array_element))
    (if Fire
      (set `/Game/Spacey_BP/Enemies/BP_EnemyGun1.Parent` self _asbp_enemy_gun_1)
      (`/Game/Spacey_BP/Enemies/BP_EnemyGun1.Shoot` _asbp_enemy_gun_1)
      (set `/Game/Spacey_BP/Enemies/BP_EnemyGun1.bLoop?` true _asbp_enemy_gun_1)
      (else
        (set `/Game/Spacey_BP/Enemies/BP_EnemyGun1.bLoop?` false _asbp_enemy_gun_1)))))

(fn `SetFireRates`
  (params (`Fast?` :type Boolean))
  (if `Fast?`
    (for _array_element (`self.GetAllChildActors` true)
      (bind _asbp_enemy_gun_1 (cast `/Game/Spacey_BP/Enemies/BP_EnemyGun1` _array_element))
      (set `/Game/Spacey_BP/Enemies/BP_EnemyGunParent.FireRate` 0.05 _asbp_enemy_gun_1))
    (else
      (for _array_element_2 (`self.GetAllChildActors` true)
        (bind _asbp_enemy_gun_1_2 (cast `/Game/Spacey_BP/Enemies/BP_EnemyGun1` _array_element_2))
        (set `/Game/Spacey_BP/Enemies/BP_EnemyGunParent.FireRate` 0.5 _asbp_enemy_gun_1_2)))))

(fn `UserConstructionScript`
  (`parent.UserConstructionScript`))