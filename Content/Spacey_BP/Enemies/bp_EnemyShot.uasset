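; Enemy projectile that plays a fire sound on spawn, moves at its configured speed and dies on impact.
; BeginPlay records the player ship's height, then after a short delay enables Tick, which eases the shot's Z onto that height at a fixed rate and switches Tick off once aligned.
; Overlapping the player ship, except its Sight component, calls DeathEvent immediately, while blocking hits call it after a brief delay.
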(event `self.ReceiveBeginPlay`
  (bind _projectilemovement (`self.ProjectileMovement`))
  (`parent.ReceiveBeginPlay`)
  (bind _asbp_player_ship (cast `/Game/Spacey_BP/Player/BP_PlayerShip` (`GameplayStatics.GetPlayerPawn` 0)))
  (bind (_returnvalue_x _returnvalue_y _returnvalue_z) (`KismetMathLibrary.BreakVector` (`self.K2_GetActorLocation` _asbp_player_ship)))
  (set `self.TargetZ` _returnvalue_z)
  (bind _output_get (set `ProjectileMovementComponent.InitialSpeed` (`self.Speed`) _projectilemovement))
  (set `ProjectileMovementComponent.MaxSpeed` _output_get _projectilemovement)
  (`GameplayStatics.PlaySoundAtLocation` "/Game/Spacey/Audio/SFX/Bullets/SFX_Fire_4_.SFX_Fire_4_" (`self.K2_GetActorLocation`) (struct) 1.0 1.0 0.0 null null null)
  (`KismetSystemLibrary.Delay` 0.1)
  (`self.SetActorTickEnabled` true))

(event `self.ReceiveTick`
  (params (DeltaSeconds :type "Float (single-precision)"))
  (`parent.ReceiveTick` DeltaSeconds)
  (`self.UpdateZ`))

(event `self.Sphere.OnComponentHit`
  (params (HitComponent :type "PrimitiveComponent Object Reference") (OtherActor :type "Actor Object Reference") (OtherComp :type "PrimitiveComponent Object Reference") (NormalImpulse :type "Vector Structure") (Hit :type "HitResult Structure (by ref)"))
  (`KismetSystemLibrary.Delay` 0.2)
  (`self.DeathEvent` true))

(event `self.Sphere.OnComponentBeginOverlap`
  (params (OverlappedComponent :type "PrimitiveComponent Object Reference") (OtherActor :type "Actor Object Reference") (OtherComp :type "PrimitiveComponent Object Reference") (OtherBodyIndex :type Integer) (bFromSweep :type Boolean) (SweepResult :type "HitResult Structure (by ref)"))
  (bind _asbp_player_ship (cast `/Game/Spacey_BP/Player/BP_PlayerShip` OtherActor))
  (if (!= OtherComp (`PlayerShipBase.Sight` _asbp_player_ship))
    (`self.DeathEvent` false)))

(event `UpdateZ`
  (bind (_returnvalue_x _returnvalue_y _returnvalue_z) (`KismetMathLibrary.BreakVector` (`self.K2_GetActorLocation`)))
  (bind (_returnvalue_x_2 _returnvalue_y_2 _returnvalue_z_2) (`KismetMathLibrary.BreakVector` (`self.K2_GetActorLocation`)))
  (bind (_returnvalue_x_3 _returnvalue_y_3) (`KismetMathLibrary.BreakVector` (`self.K2_GetActorLocation`)))
  (bind _returnvalue (`StaticsLibrary.Approach` _returnvalue_z_2 (`self.TargetZ`) (* (`GameplayStatics.GetWorldDeltaSeconds`) 500.0)))
  (`self.K2_SetActorLocation` (`KismetMathLibrary.MakeVector` _returnvalue_x_3 _returnvalue_y_3 _returnvalue))
  (if (== (`self.TargetZ`) _returnvalue_z)
    (`self.SetActorTickEnabled` false)))

(fn `UserConstructionScript`
  (`parent.UserConstructionScript`))