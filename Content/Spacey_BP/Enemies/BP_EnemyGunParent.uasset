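; Base enemy gun Blueprint that spawns bullets and repeats fire while its firing state is on.
; SetFire toggles IsFiring, calling FireEvent and printing a debug message when firing starts.
; FireEvent spawns the Bullet class at the Arrow component's location and rotation, scaled by BulletSize, and plays a sound.
; A CanShoot gate and FireRate delay space the shots, with FireEvent calling itself again while firing continues.
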(event `self.ReceiveBeginPlay`)

(event `SetFire`
  (params (`Fire?` :type Boolean))
  (if `Fire?`
    (if (== (`self.bIsFiring`) false)
      (set `self.bIsFiring` true)
      (`self.FireEvent`)
      (`KismetSystemLibrary.PrintString` "Boom"))
    (else
      (set `self.bIsFiring` false))))

(event `FireEvent`
  (bind _arrow (`self.Arrow`))
  (if (`self.bCanShoot`)
    (bind _returnvalue (`|SpawnActorFromClass` (`self.Bullet`) (`KismetMathLibrary.MakeTransform` (`SceneComponent.K2_GetComponentLocation` _arrow) (`SceneComponent.K2_GetComponentRotation` _arrow) (`self.BulletSize`)) "Undefined" "OverrideRootScale" null null))
    (`/Engine/EditorBlueprintResources/StandardMacros.IsValid` _returnvalue
      (:`Is Valid`
        (set `self.bCanShoot` false)
        (`|ExecutionSequence`
          (:`then_0`
            (`KismetSystemLibrary.Delay` (`self.FireRate`))
            (set `self.bCanShoot` true)
            (if (`self.bIsFiring`)
              (`self.FireEvent`)))
          (:`then_1`
            (`GameplayStatics.PlaySoundAtLocation` (`self.Sound`) (`self.K2_GetActorLocation`) (struct) 0.005 0.5 0.0 null null null)))))))

(fn `UserConstructionScript`)