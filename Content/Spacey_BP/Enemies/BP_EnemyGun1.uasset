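; Enemy gun Blueprint that fires bullets from its Arrow component, using its parent BP_EnemyShipBasic to check sight of the player.
; Shoot spawns a bullet with set lifetime and damage, its size scaled by SpawnScale at BeginPlay.
; A failed sight check blocks the shot by clearing the CS cooldown flag.
; Either outcome waits FireRate before re-enabling CS and, when Loop is set, calling Shoot again.
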(event `self.ReceiveBeginPlay`
  (`parent.ReceiveBeginPlay`)
  (set `self.BulletSize` (* (`self.BulletSize`) (`self.SpawnScale`))))

(event `Shoot`
  (bind _arrow (`self.Arrow`))
  (`|ExecutionSequence`
    (:`then_0`
      (bind _asbp_enemy_ship_basic (cast `/Game/Spacey_BP/Enemies/BP_EnemyShipBasic` (`self.Parent`)))
      (bind _returnvalue (`EnemyShipBase.InLineOfSight` _asbp_enemy_ship_basic (`self.K2_GetActorLocation` (`GameplayStatics.GetPlayerPawn` 0)) false))
      (if (not _returnvalue)
        (set `self.bCS` false)
        (`KismetSystemLibrary.Delay` (`self.FireRate`))
        (set `self.bCS` true)
        (if (`self.bLoop?`)
          (`self.Shoot`))))
    (:`then_1`
      (if (`self.bCS`)
        (bind _returnvalue_2 (`|SpawnActorFromClass` (`self.Bullet`) (`KismetMathLibrary.MakeTransform` (`SceneComponent.K2_GetComponentLocation` _arrow) (`SceneComponent.K2_GetComponentRotation` _arrow) (`self.BulletSize`)) "Undefined" "OverrideRootScale" null null))
        (set `/Game/Spacey_BP/BP_Shot_Parent.Lifetime` (`self.BulletLifeTime`) _returnvalue_2)
        (set `/Game/Spacey_BP/BP_Shot_Parent.Damage` (`self.Damage`) _returnvalue_2)
        (set `self.bCS` false)
        (`KismetSystemLibrary.Delay` (`self.FireRate`))
        (set `self.bCS` true)
        (if (`self.bLoop?`)
          (`self.Shoot`))))
    (:`then_2`
      (if (`self.WasRecentlyRendered` 0.2)
        _))))

(event `self.FireEvent`)

(fn `UserConstructionScript`
  (`parent.UserConstructionScript`))