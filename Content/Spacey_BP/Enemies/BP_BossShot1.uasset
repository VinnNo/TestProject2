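; BP_BossShot1 is a boss projectile that homes in on the player ship and splits into smaller shots when hit.
; On BeginPlay it sets the player ship's root as the homing target of its ProjectileMovement.
; When its sphere overlaps a BP_Ship_Shot other than itself, it spawns five Bp_EnemyShot1 actors at its Arrow components' transforms, then destroys itself.
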(event `self.ReceiveBeginPlay`
  (bind _projectilemovement (`self.ProjectileMovement`))
  (`parent.ReceiveBeginPlay`)
  (bind _asbp_player_ship (cast `/Game/Spacey_BP/Player/BP_PlayerShip` (`GameplayStatics.GetPlayerPawn` 0)))
  (`/Engine/EditorBlueprintResources/StandardMacros.IsValid` _asbp_player_ship
    (:`Is Valid`
      (set `ProjectileMovementComponent.HomingTargetComponent` (`Actor.RootComponent` _asbp_player_ship) _projectilemovement)
      (set `ProjectileMovementComponent.bIsHomingProjectile` true _projectilemovement))))

(event `self.Sphere.OnComponentBeginOverlap`
  (params (OverlappedComponent :type "PrimitiveComponent Object Reference") (OtherActor :type "Actor Object Reference") (OtherComp :type "PrimitiveComponent Object Reference") (OtherBodyIndex :type Integer) (bFromSweep :type Boolean) (SweepResult :type "HitResult Structure (by ref)"))
  (bind _asbp_ship_shot (cast `/Game/Spacey_BP/BP_Ship_Shot` OtherActor))
  (if (!= _asbp_ship_shot self)
    (`|ExecutionSequence`
      (:`then_0`
        (`|SpawnActorFromClass` "/Game/Spacey_BP/Enemies/bp_EnemyShot1.bp_EnemyShot1_C" (`SceneComponent.K2_GetComponentToWorld` (`self.Arrow`)) "Undefined" "OverrideRootScale" null null))
      (:`then_1`
        (`|SpawnActorFromClass` "/Game/Spacey_BP/Enemies/bp_EnemyShot1.bp_EnemyShot1_C" (`SceneComponent.K2_GetComponentToWorld` (`self.Arrow1`)) "Undefined" "OverrideRootScale" null null))
      (:`then_2`
        (`|SpawnActorFromClass` "/Game/Spacey_BP/Enemies/bp_EnemyShot1.bp_EnemyShot1_C" (`SceneComponent.K2_GetComponentToWorld` (`self.Arrow2`)) "Undefined" "OverrideRootScale" null null))
      (:`then_3`
        (`|SpawnActorFromClass` "/Game/Spacey_BP/Enemies/bp_EnemyShot1.bp_EnemyShot1_C" (`SceneComponent.K2_GetComponentToWorld` (`self.Arrow3`)) "Undefined" "OverrideRootScale" null null))
      (:`then_4`
        (`|SpawnActorFromClass` "/Game/Spacey_BP/Enemies/bp_EnemyShot1.bp_EnemyShot1_C" (`SceneComponent.K2_GetComponentToWorld` (`self.Arrow4`)) "Undefined" "OverrideRootScale" null null))
      (:`then_5`
        (`self.K2_DestroyActor`)))))

(fn `UserConstructionScript`
  (`parent.UserConstructionScript`))