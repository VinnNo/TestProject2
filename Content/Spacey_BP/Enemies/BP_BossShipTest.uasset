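; BP_BossShipTest is a test boss enemy ship that inherits its core behavior from a parent class.
; BeginPlay, Tick, player detection, patrol timer and state change events all pass straight to the parent.
; Its own wiring routes ship mesh overlaps to TakeDamage, Sight component overlaps to SightEntered and SightLeft, and Health depletion to DoDeath.
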(event `self.ReceiveTick`
  (params (DeltaSeconds :type "Float (single-precision)"))
  (`parent.ReceiveTick` DeltaSeconds))

(event `self.ReceiveBeginPlay`
  (`parent.ReceiveBeginPlay`))

(event `self.FoundPlayer`
  (`parent.FoundPlayer`))

(event `self.PatrolTimerUp`
  (`parent.PatrolTimerUp`))

(event `self.OnStateChanged`
  (`parent.OnStateChanged`))

(event `self.ShipMeshComponent.OnComponentBeginOverlap`
  (params (OverlappedComponent :type "PrimitiveComponent Object Reference") (OtherActor :type "Actor Object Reference") (OtherComp :type "PrimitiveComponent Object Reference") (OtherBodyIndex :type Integer) (bFromSweep :type Boolean) (SweepResult :type "HitResult Structure (by ref)"))
  (`self.TakeDamage` OtherActor))

(event `self.Sight.OnComponentBeginOverlap`
  (params (OverlappedComponent :type "PrimitiveComponent Object Reference") (OtherActor :type "Actor Object Reference") (OtherComp :type "PrimitiveComponent Object Reference") (OtherBodyIndex :type Integer) (bFromSweep :type Boolean) (SweepResult :type "HitResult Structure (by ref)"))
  (`self.SightEntered` OtherActor OtherComp))

(event `self.Sight.OnComponentEndOverlap`
  (params (OverlappedComponent :type "PrimitiveComponent Object Reference") (OtherActor :type "Actor Object Reference") (OtherComp :type "PrimitiveComponent Object Reference") (OtherBodyIndex :type Integer))
  (`self.SightLeft` OtherActor OtherComp))

(event `self.Health.OnHealthDepleted`
  (`self.Do Death`))

(fn `UserConstructionScript`
  (`parent.UserConstructionScript`))