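; Test enemy for the spaceship game that detects, chases and shoots the player ship, takes shot damage and bursts into particles on death.
; A sight sphere plus line trace sets the found state, and a retriggerable delay clears it after the player leaves.
; Tick yaws toward the player and fires child gun actors when in sight, while AIMoveTo handles movement and retries on failure.
; Health changes also trigger pursuit.
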(event `self.ReceiveBeginPlay`
  (bind _asbp_player_ship (cast `/Game/Spacey_BP/Player/BP_PlayerShip` (`GameplayStatics.GetPlayerPawn` 0)))
  (set `self.Player` _asbp_player_ship)
  (set `self.AcceptanceFound` (/ (`SphereComponent.GetScaledSphereRadius` (`self.Sight_Sphere`)) 2.0)))

(event `self.ReceiveTick`
  (params (DeltaSeconds :type "Float (single-precision)"))
  (`|ExecutionSequence`
    (:`then_0`
      (if (and (== (`self.bCancelingAI`) false) (`self.FoundHim`))
        (bind _asbp_player_ship (cast `/Game/Spacey_BP/Player/BP_PlayerShip` (`GameplayStatics.GetPlayerPawn` 0)))
        (set `self.targetLocation` (`self.K2_GetActorLocation` _asbp_player_ship))
        (else
          (set `self.targetLocation` (`self.K2_GetActorLocation`)))))
    (:`then_1`
      (if (`self.FoundHim`)
        (`self.RotateTowards`)
        (set `self.Acceptance` (`self.AcceptanceFound`))
        (if (`self.In Line Of Sight` (`self.targetLocation`))
          (`self.SetFiring` true))
        (else
          (set `self.Acceptance` (`self.AcceptanceLost`)))))))

(event `StartAI`
  (`ActorComponent.SetActive` (`self.ParticleSystem1`) (`self.bCancelingAI`) false)
  (`ActorComponent.SetActive` (`self.ParticleSystem`) (`self.bCancelingAI`) false)
  (set `self.IsAi` true)
  (`|AIMoveTo` self (`self.targetLocation`) (`self.TargetActor`)
    (:`then`
      (`KismetSystemLibrary.PrintString` (`KismetStringLibrary.Conv_VectorToString` (`self.targetLocation`))))
    (:`OnSuccess`
      (set `self.IsAi` false))
    (:`OnFail`
      (set `self.IsAi` false)
      (`KismetSystemLibrary.Delay` 0.2)
      (`self.StartAI`))))

(event `CancelAI`
  (set `self.TargetActor` self)
  (`self.StartAI`))

(event `self.Sight_Sphere.OnComponentBeginOverlap`
  (params (OverlappedComponent :type "PrimitiveComponent Object Reference") (OtherActor :type "Actor Object Reference") (OtherComp :type "PrimitiveComponent Object Reference") (OtherBodyIndex :type Integer) (bFromSweep :type Boolean) (SweepResult :type "HitResult Structure (by ref)"))
  (if (`self.In Line Of Sight` (`self.targetLocation`))
    (bind _asbp_player_ship (cast `/Game/Spacey_BP/Player/BP_PlayerShip` OtherActor))
    (set `self.Player` _asbp_player_ship)
    (`self.CancelAI`)
    (set `self.FoundHim` true)
    (set `self.TargetActor` (`GameplayStatics.GetPlayerPawn` 0))))

(event `self.Sight_Sphere.OnComponentEndOverlap`
  (params (OverlappedComponent :type "PrimitiveComponent Object Reference") (OtherActor :type "Actor Object Reference") (OtherComp :type "PrimitiveComponent Object Reference") (OtherBodyIndex :type Integer))
  (bind _asbp_player_ship (cast `/Game/Spacey_BP/Player/BP_PlayerShip` OtherActor))
  (set `self.Player` _asbp_player_ship)
  (`self.StartAI`)
  (`KismetSystemLibrary.RetriggerableDelay` (`self.RememberTargetTime`))
  (`self.CancelAI`)
  (set `self.FoundHim` false))

(event `RotateTowards`
  (`SceneComponent.K2_SetWorldRotation` (`self.CapsuleComponent`) (`KismetMathLibrary.MakeRotator` 0.0 0.0 (+ (.yaw (`KismetMathLibrary.FindLookAtRotation` (`SceneComponent.K2_GetComponentLocation` (`self.CapsuleComponent`)) (`self.K2_GetActorLocation` (`self.Player`)))) 0.0)) false false))

(event `self.StaticMesh.OnComponentBeginOverlap`
  (params (OverlappedComponent :type "PrimitiveComponent Object Reference") (OtherActor :type "Actor Object Reference") (OtherComp :type "PrimitiveComponent Object Reference") (OtherBodyIndex :type Integer) (bFromSweep :type Boolean) (SweepResult :type "HitResult Structure (by ref)"))
  (bind _asbp_shot_parent (cast `/Game/Spacey_BP/BP_Shot_Parent` OtherActor))
  (`HealthComponent.DecrementHealth` (`self.Health`) (`/Game/Spacey_BP/BP_Shot_Parent.Damage` _asbp_shot_parent)))

(event `self.Health.OnHealthChanged`
  (`self.StartAI`)
  (set `self.FoundHim` true)
  (set `self.bCancelingAI` false))

(event `self.Health.OnHealthDepleted`
  (for _ (range (+ (`self.DeathParticleCount`) 1))
    (`GameplayStatics.SpawnEmitterAtLocation` "/Game/Spacey/Particles/p_EnemyShotDeath.p_EnemyShotDeath" (+ (`self.K2_GetActorLocation`) (`self.RandomIzeVector` (`self.DeathParticleRange`))) (struct) (3.0 3.0 3.0)))
  (`self.K2_DestroyActor`))

(fn `In Line Of Sight`
  (params (Target :type "Vector Structure"))
  (returns (Found :type Boolean))
  (locals (bInLine :type Boolean))
  (bind _outhit (`KismetSystemLibrary.LineTraceSingle` :`Start` (`self.K2_GetActorLocation`) :`End` Target :`TraceChannel` "TraceTypeQuery1" :`DrawDebugType` "ForOneFrame" :`TraceColor` (struct :`R` 0.129445 :`G` 1.0 :`B` 0.015198 :`A` 1.0) :`TraceHitColor` (struct :`R` 1.0 :`A` 1.0)))
  (cast `/Game/Spacey_BP/Player/BP_PlayerShip` (`.HitActor` (`GameplayStatics.BreakHitResult` _outhit))
    (:`then`
      (set `local.bInLine` true))
    (:`CastFailed`
      (set `local.bInLine` false)))
  (return (`local.bInLine`)))

(fn `RandomIzeVector`
  (params (in :type "Vector Structure"))
  (returns (Out :type "Vector Structure"))
  (return (`KismetMathLibrary.MakeVector` (`KismetMathLibrary.RandomFloatInRange` (- 0.0 in_X) in_X) (`KismetMathLibrary.RandomFloatInRange` (- 0.0 in_Y) in_Y) (`KismetMathLibrary.RandomFloatInRange` (- 0.0 in_Z) in_Z))))

(fn `SetFiring`
  (params (`Fire?` :type Boolean))
  (locals (Fire :type Boolean))
  (set `local.Fire` `Fire?`)
  (for _array_element (`self.GetAllChildActors` true)
    (bind _asbp_enemy_gun_1 (cast `/Game/Spacey_BP/Enemies/BP_EnemyGun1` _array_element))
    (`/Game/Spacey_BP/Enemies/BP_EnemyGun1.Shoot` _asbp_enemy_gun_1))
  (set `self.bIsFiring` (`local.Fire`)))

(fn `UserConstructionScript`
  (`self.K2_AttachToComponent` null "None" "KeepRelative" "KeepRelative" "KeepRelative"))