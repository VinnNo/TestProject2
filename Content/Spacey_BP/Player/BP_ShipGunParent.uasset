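; Parent Blueprint for player ship guns that spawns projectiles from its Arrow with auto-fire while the trigger is held.
; Shortly after BeginPlay it normalizes fire rate and power into a shot delay and projectile damage.
; SetShot starts firing outside Map_Menu, and FireEvent re-triggers itself after delay plus cooldown until StopShot.
; Each shot sets projectile damage and speed and plays a sound, with volume lowered on the menu map.
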(event `self.ReceiveBeginPlay`
  (`KismetSystemLibrary.Delay` 0.15)
  (`self.SetGunStats`))

(event `SetGunStats`
  (set `self.Fire` (/ (`self.FireRate`) (`self.FireRateMax`)))
  (set `self.Power` (/ (`self.FirePower`) (`self.FirePowerMax`)))
  (set `self.FireTime` (/ (- 1.0 (`self.Fire`)) 10.0)))

(event `SetShot`
  (bind _returnvalue (`GameplayStatics.GetCurrentLevelName` true))
  (if (and (== (`self.bIsFiring`) false) (`KismetStringLibrary.NotEqual_StrStr` _returnvalue "Map_Menu"))
    (set `self.bIsFiring` true)
    (`self.FireEvent`)))

(event `StopShot`
  (set `self.bIsFiring` false))

(event `FireEvent`
  (bind _arrow (`self.Arrow`))
  (if (`self.bCanShoot`)
    (bind _returnvalue (`|SpawnActorFromClass` (`self.Shot`) (`KismetMathLibrary.MakeTransform` (`SceneComponent.K2_GetComponentLocation` _arrow) (`SceneComponent.K2_GetComponentRotation` _arrow) (`self.BulletSize`)) "Undefined" "OverrideRootScale" null null))
    (`/Engine/EditorBlueprintResources/StandardMacros.IsValid` _returnvalue
      (:`Is Valid`
        (set `/Game/Spacey_BP/BP_Shot_Parent.Damage` (`self.Power`) _returnvalue)
        (bind _projectilemovement (`/Game/Spacey_BP/BP_Shot_Parent.ProjectileMovement` _returnvalue))
        (bind _output_get (set `ProjectileMovementComponent.InitialSpeed` (`self.BulletSpeed`) _projectilemovement))
        (set `ProjectileMovementComponent.MaxSpeed` _output_get _projectilemovement)
        (set `self.bCanShoot` false)
        (`|ExecutionSequence`
          (:`then_0`
            (`KismetSystemLibrary.Delay` (+ (`self.FireTime`) (`self.cooldown`)))
            (set `self.bCanShoot` true)
            (if (`self.bIsFiring`)
              (`self.FireEvent`)))
          (:`then_1`
            (bind _returnvalue_2 (`GameplayStatics.GetCurrentLevelName` true))
            (if (`KismetStringLibrary.EqualEqual_StrStr` _returnvalue_2 "Map_Menu")
              (set `self.Volume` 0.35)))
          (:`then_2`
            (`GameplayStatics.PlaySoundAtLocation` (`self.SFX`) (`self.K2_GetActorLocation`) (struct) (`self.Volume`) 1.0 0.0 null null null)))))))

(fn `UserConstructionScript`)