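; Player ship shield actor, a randomly spinning inner and outer shell with a looping running sound.
; Enemy shot hits on the inner shell subtract the shot's damage from its remaining shield time and play a block sound.
; Half and low health events swap both shells' materials to show depletion.
; TurnOffShield resets the player ship's shield time, triggers its startup delay and destroys the actor.
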(event `self.ReceiveBeginPlay`
  (set `RotatingMovementComponent.RotationRate` (`KismetMathLibrary.MakeRotator` (`KismetMathLibrary.RandomFloatInRange` -180.0 180.0) (`KismetMathLibrary.RandomFloatInRange` -180.0 180.0) (`KismetMathLibrary.RandomFloatInRange` -180.0 180.0)) (`self.RotatingMovement`))
  (bind _returnvalue (`GameplayStatics.SpawnSoundAttached` "/Game/Spacey/Audio/SFX/Shields/SFX_Shields_Running.SFX_Shields_Running" (`self.ShieldInner`) "None" (0.0 0.0 0.0) (struct) "KeepRelativeOffset" true 1.0 1.0 0.0 null null false))
  (set `self.SFX` _returnvalue))

(event `self.TurnOffShield`
  (bind _asbp_player_ship (cast `/Game/Spacey_BP/Player/BP_PlayerShip` (`GameplayStatics.GetPlayerPawn` 0)))
  (set `PlayerShipBase.ShieldTimeCurrent` -1.0 _asbp_player_ship)
  (`/Game/Spacey_BP/Player/BP_PlayerShip.ShieldStartupDelay` _asbp_player_ship)
  (`self.K2_DestroyActor`))

(event `self.ShieldInner.OnComponentHit`
  (params (HitComponent :type "PrimitiveComponent Object Reference") (OtherActor :type "Actor Object Reference") (OtherComp :type "PrimitiveComponent Object Reference") (NormalImpulse :type "Vector Structure") (Hit :type "HitResult Structure (by ref)"))
  (bind _asbp_enemy_shot (cast `/Game/Spacey_BP/Enemies/bp_EnemyShot` OtherActor))
  (set `self.ShieldTimeCurrent` (- (`self.ShieldTimeCurrent`) (`/Game/Spacey_BP/BP_Shot_Parent.Damage` _asbp_enemy_shot)))
  (`GameplayStatics.PlaySoundAtLocation` "/Game/Spacey/Audio/SFX/Shields/SFX_Shields_Block.SFX_Shields_Block" (`self.K2_GetActorLocation`) (struct) 1.0 1.0 0.0 null null null))

(event `self.OnLowHealth`
  (`PrimitiveComponent.SetMaterial` (`self.ShieldInner`) 0 "/Game/Spacey/Materials/PlayerShip/mat_Ship_ShieldsLow_Inst.mat_Ship_ShieldsLow_Inst")
  (`PrimitiveComponent.SetMaterial` (`self.ShieldOuter`) 0 "/Game/Spacey/Materials/PlayerShip/mat_Ship_ShieldsLow_Outer_Inst.mat_Ship_ShieldsLow_Outer_Inst"))

(event `self.OnHalfHealth`
  (`PrimitiveComponent.SetMaterial` (`self.ShieldInner`) 0 "/Game/Spacey/Materials/PlayerShip/mat_Ship_ShieldsHalf_Inst1.mat_Ship_ShieldsHalf_Inst1")
  (`PrimitiveComponent.SetMaterial` (`self.ShieldOuter`) 0 "/Game/Spacey/Materials/PlayerShip/mat_Ship_ShieldsHalf_Outer_Inst.mat_Ship_ShieldsHalf_Outer_Inst"))

(fn `UserConstructionScript`)