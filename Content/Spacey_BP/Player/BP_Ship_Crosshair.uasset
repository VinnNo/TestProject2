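; Player ship crosshair actor that switches between an aiming look and a locked-on look.
; SetLock toggles visibility of the Aim and LockedOn components.
; On lock it checks for zero yaw rate, then spins through RotatingMovement in a random direction; on unlock it stops and resets rotation.
; The Sphere overlap events are empty, and older overlap-based lock logic is left disconnected.
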(event `self.Sphere.OnComponentBeginOverlap`
  (params (OverlappedComponent :type "PrimitiveComponent Object Reference") (OtherActor :type "Actor Object Reference") (OtherComp :type "PrimitiveComponent Object Reference") (OtherBodyIndex :type Integer) (bFromSweep :type Boolean) (SweepResult :type "HitResult Structure (by ref)")))

(event `self.Sphere.OnComponentEndOverlap`
  (params (OverlappedComponent :type "PrimitiveComponent Object Reference") (OtherActor :type "Actor Object Reference") (OtherComp :type "PrimitiveComponent Object Reference") (OtherBodyIndex :type Integer)))

(event `SetLock`
  (params (`LockedOn?` :type Boolean))
  (bind (_rotationrate_roll _rotationrate_pitch _rotationrate_yaw) (`KismetMathLibrary.BreakRotator` (`RotatingMovementComponent.RotationRate` (`self.RotatingMovement`))))
  (if `LockedOn?`
    (`SceneComponent.SetVisibility` (`self.LockedOn`) true false)
    (`SceneComponent.SetVisibility` (`self.Aim`) false false)
    (if (== _rotationrate_yaw 0.0)
      (`self.RandomizeRotation`)
      (set `RotatingMovementComponent.RotationRate` (`self.RotationYaw`) (`self.RotatingMovement`)))
    (else
      (`SceneComponent.SetVisibility` (`self.LockedOn`) false false)
      (`SceneComponent.SetVisibility` (`self.Aim`) true false)
      (set `RotatingMovementComponent.RotationRate` (struct) (`self.RotatingMovement`))
      (`self.K2_SetActorRotation` (struct)))))

(event `RandomizeRotation`
  (if (> (`KismetMathLibrary.RandomFloatInRange` 1.0 100.0) 50.0)
    (set `self.RotationYaw` (struct :`Yaw` 360.0))
    (else
      (set `self.RotationYaw` (struct :`Yaw` -360.0)))))

(fn `UserConstructionScript`)