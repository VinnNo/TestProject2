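; BP_Player holds the player's persistent state in a space game: money, left and right guns, and ship health.
; SaveController writes these to a BP_SaveGame in a slot named by PawnTag.
; LoadController restores them, or creates the save through SaveController if none exists.
; Nothing here calls LoadController on a live path, and saving of ship location and rotation is left unconnected.
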(event `self.ReceiveBeginPlay`)

(event `SaveController`
  (bind _returnvalue (`GameplayStatics.CreateSaveGameObject` "/Game/Spacey_BP/BP_SaveGame.BP_SaveGame_C"))
  (set `/Game/Spacey_BP/BP_SaveGame.Money` (`self.Money`) _returnvalue)
  (set `/Game/Spacey_BP/BP_SaveGame.PlayerGunLeft` (`self.GunLeft`) _returnvalue)
  (set `/Game/Spacey_BP/BP_SaveGame.PlayerGunRight` (`self.GunRight`) _returnvalue)
  (set `/Game/Spacey_BP/BP_SaveGame.ShipHealthCurrent` (`self.ShipHealth`) _returnvalue)
  (bind _returnvalue_2 (`GameplayStatics.SaveGameToSlot` _returnvalue (`self.PawnTag`)))
  (bind _output_get (set `self.bSaved` _returnvalue_2))
  (if _output_get
    (`KismetSystemLibrary.PrintString` "PawnSaved")))

(event `LoadController`
  (bind _pawntag (`self.PawnTag`))
  (bind _returnvalue (`GameplayStatics.DoesSaveGameExist` _pawntag))
  (if _returnvalue
    (bind _returnvalue_2 (`GameplayStatics.LoadGameFromSlot` _pawntag))
    (bind _asbp_save_game (cast `/Game/Spacey_BP/BP_SaveGame` _returnvalue_2))
    (set `self.Money` (`/Game/Spacey_BP/BP_SaveGame.Money` _asbp_save_game))
    (set `self.GunRight` (`/Game/Spacey_BP/BP_SaveGame.PlayerGunRight` _asbp_save_game))
    (set `self.GunLeft` (`/Game/Spacey_BP/BP_SaveGame.PlayerGunLeft` _asbp_save_game))
    (set `self.ShipHealth` (`/Game/Spacey_BP/BP_SaveGame.ShipHealthCurrent` _asbp_save_game))
    (`KismetSystemLibrary.PrintString` "PawnLoaded")
    (else
      (`self.SaveController`))))

(fn `UserConstructionScript`)