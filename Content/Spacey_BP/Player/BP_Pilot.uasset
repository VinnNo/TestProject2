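; Player pilot that walks the ship interior and opens station menus to buy gun, shield and ship-system upgrades.
; Movement pins height to the starting Z, while menu input is routed by MenuNumber to the current widget.
; Closing an upgrade menu copies its stats and money back to the pilot and HUD.
; The "Shared" save slot loads on BeginPlay and is written on station confirm, RetrieveAll or exit to Map_Menu.
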(event `InputAction|MenuLeft`
  (params (Key :type "Key Structure"))
  (:`Pressed`
    (switch `int` (`self.MenuNumber`)
      (:`0`
        (bind _asbp_widget_station_pilot (cast `/Game/Spacey_BP/UI/Ship_Interior/BP_Widget_Station_Pilot` (`self.CurrentMenu`)))
        (`/Game/Spacey_BP/UI/Ship_Interior/BP_Widget_Station_Pilot.SwitchMenuSelection` _asbp_widget_station_pilot))
      (:`1`
        (bind _asbp_guns_widget (cast `/Game/Spacey_BP/UI/Ship_Interior/BP_Guns_Widget` (`self.CurrentMenu`)))
        (if (== (`WidgetGuns.SelectedUpgrade` _asbp_guns_widget) 2)
          (`/Game/Spacey_BP/UI/Ship_Interior/BP_Guns_Widget.SetUpgradeSelection` _asbp_guns_widget 1)
          (else
            (`/Game/Spacey_BP/UI/Ship_Interior/BP_Guns_Widget.SetUpgradeSelection` _asbp_guns_widget 2))))
      (:`2`
        (bind _asbp_shields_widget (cast `/Game/Spacey_BP/UI/Ship_Interior/BP_Shields_Widget` (`self.CurrentMenu`)))
        (bind _selectedupgrade (`WidgetShields.SelectedUpgrade` _asbp_shields_widget))
        (if (== _selectedupgrade 1)
          (`/Game/Spacey_BP/UI/Ship_Interior/BP_Shields_Widget.SwitchUpgradeSelection` _asbp_shields_widget 4 1)
          (else
            (`/Game/Spacey_BP/UI/Ship_Interior/BP_Shields_Widget.SwitchUpgradeSelection` _asbp_shields_widget (- _selectedupgrade 1) _selectedupgrade))))
      (:`3`
        (bind _asbp_ship_systems_widget (cast `/Game/Spacey_BP/UI/Ship_Interior/BP_Ship_Systems_Widget` (`self.CurrentMenu`)))
        (bind _selectedupgrade_2 (`WidgetShipSystems.SelectedUpgrade` _asbp_ship_systems_widget))
        (if (== _selectedupgrade_2 1)
          (`/Game/Spacey_BP/UI/Ship_Interior/BP_Ship_Systems_Widget.SwitchUpgradeSelection` _asbp_ship_systems_widget 4)
          (else
            (`/Game/Spacey_BP/UI/Ship_Interior/BP_Ship_Systems_Widget.SwitchUpgradeSelection` _asbp_ship_systems_widget (- _selectedupgrade_2 1))))))))

(event `SpawnWidgets`
  (bind _returnvalue (`GameplayStatics.GetPlayerController` 0))
  (`|ExecutionSequence`
    (:`then_0`
      (`WidgetLayoutLibrary.RemoveAllWidgets`)
      (`PlayerController.ActivateTouchInterface` _returnvalue (`self.TouchInterface`)))
    (:`then_1`
      (bind _returnvalue_2 (`|CreateWidget` "/Game/Spacey_BP/UI/Ship_Interior/WBP_PilotHUD.WBP_PilotHUD_C" _returnvalue))
      (bind _output_get (set `self.PilotHUD` _returnvalue_2))
      (`/Game/Spacey_BP/UI/Ship_Interior/WBP_PilotHUD.SetMoney` _output_get (`self.Money`)))
    (:`then_2`
      (bind _returnvalue_3 (`|CreateWidget` "/Game/Spacey_BP/UI/WBP_WaveDisplayPilot.WBP_WaveDisplayPilot_C" _returnvalue))
      (set `self.WaveDisplay` _returnvalue_3))
    (:`then_3`
      (`UserWidget.AddToViewport` (`self.WaveDisplay`) 0)
      (`UserWidget.AddToViewport` (`self.PilotHUD`) 0))))

(event `InputAction|Accept`
  (params (Key :type "Key Structure"))
  (bind _currentmenu (`self.CurrentMenu`))
  ;[1 1 1] Menu Inputs
  (:`Pressed`
    (if (`KismetSystemLibrary.IsValid` (`self.CurrentMenu`))
      (switch `int` (`self.MenuNumber`)
        (:`0`
          (bind _asbp_game_mode_pilot (cast `/Game/Spacey_BP/BP_GameMode_Pilot` (`GameplayStatics.GetGameMode`))
            (:`then`
              (`/Game/Spacey_BP/BP_GameMode_Pilot.SaveGameMode` _asbp_game_mode_pilot))
            (:`CastFailed`
              _))
          (`self.SavePilot`)
          (bind _asbp_widget_station_pilot (cast `/Game/Spacey_BP/UI/Ship_Interior/BP_Widget_Station_Pilot` _currentmenu))
          (`/Game/Spacey_BP/UI/Ship_Interior/BP_Widget_Station_Pilot.Yes` _asbp_widget_station_pilot))
        (:`1`
          (bind _asbp_guns_widget (cast `/Game/Spacey_BP/UI/Ship_Interior/BP_Guns_Widget` _currentmenu))
          (`/Game/Spacey_BP/UI/Ship_Interior/BP_Guns_Widget.Yes` _asbp_guns_widget))
        (:`2`
          (bind _asbp_shields_widget (cast `/Game/Spacey_BP/UI/Ship_Interior/BP_Shields_Widget` _currentmenu))
          (`/Game/Spacey_BP/UI/Ship_Interior/BP_Shields_Widget.Yes` _asbp_shields_widget))
        (:`3`
          (bind _asbp_ship_systems_widget (cast `/Game/Spacey_BP/UI/Ship_Interior/BP_Ship_Systems_Widget` _currentmenu))
          (`/Game/Spacey_BP/UI/Ship_Interior/BP_Ship_Systems_Widget.Yes` _asbp_ship_systems_widget)))
      (elif (`KismetSystemLibrary.IsValid` (`self.OverlappingStation`))
        (`/Game/Spacey_BP/BP_Station_Trigger_Parent.LoadUI` (`self.OverlappingStation`) self)))))

(event `self.ReceiveBeginPlay`
  (bind (_returnvalue_x _returnvalue_y _returnvalue_z) (`KismetMathLibrary.BreakVector` (`self.K2_GetActorLocation`)))
  ;[1 1 1] Begin Play
  (set `self.StartZ` _returnvalue_z)
  (`self.LoadPilot`)
  (bind _returnvalue (`GameplayStatics.SpawnSoundAttached` "/Game/Spacey/Audio/Music/Music_Ship_Interior.Music_Ship_Interior" (`self.RootComponent`) "None" (0.0 0.0 0.0) (struct) "KeepRelativeOffset" false 1.0 1.0 0.0 null null))
  (`AudioComponent.Play` _returnvalue 0.0)
  (`self.SpawnWidgets`))

(event `InputAxis|MoveForward`
  (params (AxisValue :type "Float (single-precision)"))
  (bind (_returnvalue_x _returnvalue_y) (`KismetMathLibrary.BreakVector` (`self.K2_GetActorLocation`)))
  ;[1 1 1] All Things Movement
  ;;[1 1 1] Walk and Strafe
  (if (`self.bCanMove`)
    (`self.AddMovementInput` (`KismetMathLibrary.GetForwardVector` (`self.K2_GetActorRotation`)) AxisValue)
    (`self.K2_SetActorLocation` (`KismetMathLibrary.MakeVector` _returnvalue_x _returnvalue_y (`self.StartZ`)) :!label _label)))

(event `InputAxis|TurnUp`
  (params (AxisValue :type "Float (single-precision)"))
  ;[1 1 1] All Things Movement
  ;;[1 1 1] Joystick Look
  (if (`self.bCanMove`)
    (`self.AddControllerPitchInput` (* AxisValue (* (/ (`self.TurnSpeed`) 2.0) (`GameplayStatics.GetWorldDeltaSeconds`))))))

(event `InputAction|Back`
  (params (Key :type "Key Structure"))
  ;[1 1 1] Menu Inputs
  (:`Pressed`
    (if (`KismetSystemLibrary.IsValid` (`self.CurrentMenu`))
      (`GameplayStatics.PlaySound2D` "/Game/Spacey/Audio/SFX/Menus/Widets/drop_004.drop_004" 1.0 1.0 0.0 null null)
      (switch `int` (`self.MenuNumber`)
        (:`0`
          (bind _asbp_widget_station_pilot (cast `/Game/Spacey_BP/UI/Ship_Interior/BP_Widget_Station_Pilot` (`self.CurrentMenu`)))
          (`/Game/Spacey_BP/UI/Ship_Interior/BP_Widget_Station_Pilot.No` _asbp_widget_station_pilot))
        (:`1`
          (bind _asbp_guns_widget (cast `/Game/Spacey_BP/UI/Ship_Interior/BP_Guns_Widget` (`self.CurrentMenu`))
            (:`then`
              (if (`/Game/Spacey_BP/UI/Ship_Interior/BP_Guns_Widget.bConfirmPurchase?` _asbp_guns_widget)
                (`/Game/Spacey_BP/UI/Ship_Interior/BP_Guns_Widget.SetConfirmPanel` _asbp_guns_widget false false)
                (else
                  (`self.FetchGunStats` :!label _label_2)
                  (`Widget.RemoveFromParent` (`self.CurrentMenu`))
                  (set `self.CurrentMenu` null)
                  (`self.SetMove` true))))
            (:`CastFailed`
              (goto _label_2))))
        (:`2`
          (bind _asbp_shields_widget (cast `/Game/Spacey_BP/UI/Ship_Interior/BP_Shields_Widget` (`self.CurrentMenu`))
            (:`then`
              (if (`/Game/Spacey_BP/UI/Ship_Interior/BP_Shields_Widget.bConfirmPurchase` _asbp_shields_widget)
                (`/Game/Spacey_BP/UI/Ship_Interior/BP_Shields_Widget.SetConfirmPanel` _asbp_shields_widget false false)
                (else
                  (`self.FetchShieldValues` :!label _label_3)
                  (`Widget.RemoveFromParent` (`self.CurrentMenu`))
                  (set `self.CurrentMenu` null)
                  (`self.SetMove` true))))
            (:`CastFailed`
              (goto _label_3))))
        (:`3`
          (bind _asbp_ship_systems_widget (cast `/Game/Spacey_BP/UI/Ship_Interior/BP_Ship_Systems_Widget` (`self.CurrentMenu`))
            (:`then`
              (if (`/Game/Spacey_BP/UI/Ship_Interior/BP_Ship_Systems_Widget.bConfirmPurchase` _asbp_ship_systems_widget)
                (`/Game/Spacey_BP/UI/Ship_Interior/BP_Ship_Systems_Widget.SetConfirmPanel` _asbp_ship_systems_widget false false)
                (else
                  (`self.FetchSystemsValues` :!label _label_4)
                  (`Widget.RemoveFromParent` (`self.CurrentMenu`))
                  (set `self.CurrentMenu` null)
                  (`self.SetMove` true))))
            (:`CastFailed`
              (goto _label_4)))))
      (else
        (`self.SavePilot`)
        (`GameplayStatics.OpenLevel` "Map_Menu")))))

(event `InputAction|MenuRight`
  (params (Key :type "Key Structure"))
  (:`Pressed`
    (switch `int` (`self.MenuNumber`)
      (:`0`
        (bind _asbp_widget_station_pilot (cast `/Game/Spacey_BP/UI/Ship_Interior/BP_Widget_Station_Pilot` (`self.CurrentMenu`)))
        (`/Game/Spacey_BP/UI/Ship_Interior/BP_Widget_Station_Pilot.SwitchMenuSelection` _asbp_widget_station_pilot))
      (:`1`
        (bind _asbp_guns_widget (cast `/Game/Spacey_BP/UI/Ship_Interior/BP_Guns_Widget` (`self.CurrentMenu`)))
        (if (== (`WidgetGuns.SelectedUpgrade` _asbp_guns_widget) 1)
          (`/Game/Spacey_BP/UI/Ship_Interior/BP_Guns_Widget.SetUpgradeSelection` _asbp_guns_widget 2)
          (else
            (`/Game/Spacey_BP/UI/Ship_Interior/BP_Guns_Widget.SetUpgradeSelection` _asbp_guns_widget 1))))
      (:`2`
        (bind _asbp_shields_widget (cast `/Game/Spacey_BP/UI/Ship_Interior/BP_Shields_Widget` (`self.CurrentMenu`)))
        (bind _selectedupgrade (`WidgetShields.SelectedUpgrade` _asbp_shields_widget))
        (if (== _selectedupgrade 4)
          (`/Game/Spacey_BP/UI/Ship_Interior/BP_Shields_Widget.SwitchUpgradeSelection` _asbp_shields_widget 1 4)
          (else
            (`/Game/Spacey_BP/UI/Ship_Interior/BP_Shields_Widget.SwitchUpgradeSelection` _asbp_shields_widget (+ _selectedupgrade 1) _selectedupgrade))))
      (:`3`
        (bind _asbp_ship_systems_widget (cast `/Game/Spacey_BP/UI/Ship_Interior/BP_Ship_Systems_Widget` (`self.CurrentMenu`)))
        (bind _selectedupgrade_2 (`WidgetShipSystems.SelectedUpgrade` _asbp_ship_systems_widget))
        (if (== _selectedupgrade_2 4)
          (`/Game/Spacey_BP/UI/Ship_Interior/BP_Ship_Systems_Widget.SwitchUpgradeSelection` _asbp_ship_systems_widget 1)
          (else
            (`/Game/Spacey_BP/UI/Ship_Interior/BP_Ship_Systems_Widget.SwitchUpgradeSelection` _asbp_ship_systems_widget (+ _selectedupgrade_2 1))))))))

(event `InputAxis|TurnRight`
  (params (AxisValue :type "Float (single-precision)"))
  ;[1 1 1] All Things Movement
  ;;[1 1 1] Joystick Look
  (if (`self.bCanMove`)
    (`self.AddControllerYawInput` (* AxisValue (* (`self.TurnSpeed`) (`GameplayStatics.GetWorldDeltaSeconds`))))))

(event `InputAxis|MoveRight`
  (params (AxisValue :type "Float (single-precision)"))
  ;[1 1 1] All Things Movement
  ;;[1 1 1] Walk and Strafe
  (if (`self.bCanMove`)
    (`self.AddMovementInput` (`KismetMathLibrary.GetRightVector` (`self.K2_GetActorRotation`)) AxisValue)
    (goto _label)))

(event `InputAxis|LookUp`
  (params (AxisValue :type "Float (single-precision)"))
  ;[1 1 1] All Things Movement
  ;;[1 1 1] Mouse Look
  (if (`self.bCanMove`)
    (`self.AddControllerPitchInput` AxisValue)))

(event `SetMove`
  (params (`CanMove?` :type Boolean))
  ;[1 1 1] All Things Movement
  (bind _output_get (set `self.bCanMove` `CanMove?`))
  (if _output_get
    _))

(event `InputAxis|LookRight`
  (params (AxisValue :type "Float (single-precision)"))
  ;[1 1 1] All Things Movement
  ;;[1 1 1] Mouse Look
  (if (`self.bCanMove`)
    (`self.AddControllerYawInput` AxisValue)))

(event `InputAction|MenuDown`
  (params (Key :type "Key Structure"))
  (:`Pressed`
    (bind _asbp_guns_widget (cast `/Game/Spacey_BP/UI/Ship_Interior/BP_Guns_Widget` (`self.CurrentMenu`)))
    (`WidgetGuns.MenuSetSelectedGun` _asbp_guns_widget 2)))

(event `InputAction|MenuUp`
  (params (Key :type "Key Structure"))
  (:`Pressed`
    (bind _asbp_guns_widget (cast `/Game/Spacey_BP/UI/Ship_Interior/BP_Guns_Widget` (`self.CurrentMenu`)))
    (`WidgetGuns.MenuSetSelectedGun` _asbp_guns_widget 1)))

(event `GunsMenuUpgradeGuns`
  (params (Value :type Integer))
  (bind _asbp_widget_station_guns (cast `/Game/Spacey_BP/UI/Ship_Interior/BP_Widget_Station_Guns` (`self.CurrentMenu`)))
  (switch `int` Value
    (:`0`
      (`/Game/Spacey_BP/UI/Ship_Interior/BP_Widget_Station_Guns.UpgradeFire1` _asbp_widget_station_guns))
    (:`1`
      (`/Game/Spacey_BP/UI/Ship_Interior/BP_Widget_Station_Guns.UpgradeFire2` _asbp_widget_station_guns))
    (:`2`
      (`/Game/Spacey_BP/UI/Ship_Interior/BP_Widget_Station_Guns.UpgradePower1` _asbp_widget_station_guns))
    (:`3`
      (`/Game/Spacey_BP/UI/Ship_Interior/BP_Widget_Station_Guns.UpgradePower2` _asbp_widget_station_guns))))

(event `InputAction|Action_Debug`
  (params (Key :type "Key Structure")))

(event `RetrieveAll`
  (`self.FetchGunStats`)
  (`self.FetchShieldValues`)
  (`self.FetchSystemsValues`)
  (`self.SavePilot`)
  (bind _asbp_game_mode_pilot (cast `/Game/Spacey_BP/BP_GameMode_Pilot` (`GameplayStatics.GetGameMode`)))
  (`/Game/Spacey_BP/BP_GameMode_Pilot.SaveGameMode` _asbp_game_mode_pilot))

(event `Key|Android_Back`
  (params (Key :type "Key Structure")))

(event `Key|Escape`
  (params (Key :type "Key Structure")))

(event `FetchGunStats`
  (bind _asbp_guns_widget (cast `/Game/Spacey_BP/UI/Ship_Interior/BP_Guns_Widget` (`self.CurrentMenu`)))
  (bind (_f1 _f2 _p1 _p2 _m) (`WidgetGuns.ReturnWidgetValues` _asbp_guns_widget))
  (set `self.Fire1` _f1)
  (set `self.Fire2` _f2)
  (set `self.Power1` _p1)
  (set `self.Power2` _p2)
  (set `self.Money` _m)
  (`self.UpdatePilotHUD`))

(event `FetchShieldValues`
  (bind _asbp_shields_widget (cast `/Game/Spacey_BP/UI/Ship_Interior/BP_Shields_Widget` (`self.CurrentMenu`)))
  (bind (_outmax _outdrain _outregen _outboot _outmoney) (`WidgetShields.ReturnWidgetValues` _asbp_shields_widget))
  (set `self.ShieldMax` _outmax)
  (set `self.ShieldDrain` _outdrain)
  (set `self.ShieldRegen` _outregen)
  (set `self.ShieldBootUp` _outboot)
  (set `self.Money` _outmoney)
  (`self.UpdatePilotHUD`))

(event `UpdatePilotHUD`
  (if (`KismetSystemLibrary.IsValid` (`self.PilotHUD`))
    (`/Game/Spacey_BP/UI/Ship_Interior/WBP_PilotHUD.SetMoney` (`self.PilotHUD`) (`self.Money`))))

(event `SaveToGame`
  ;[1 1 1] Old Saves
  (bind _returnvalue (`GameplayStatics.CreateSaveGameObject` "/Game/Spacey_BP/BP_SaveGame.BP_SaveGame_C"))
  (set `/Game/Spacey_BP/BP_SaveGame.PlayerGunLeft` (`self.GunLeft`) _returnvalue)
  (set `/Game/Spacey_BP/BP_SaveGame.PlayerGunRight` (`self.GunRight`) _returnvalue)
  (set `/Game/Spacey_BP/BP_SaveGame.Money` (`self.Money`) _returnvalue)
  (bind _returnvalue_2 (`GameplayStatics.SaveGameToSlot` _returnvalue "TheGame"))
  (if _returnvalue_2
    (`KismetSystemLibrary.PrintString` "Saved To The Game")))

(event `FetchSystemsValues`
  (bind _asbp_ship_systems_widget (cast `/Game/Spacey_BP/UI/Ship_Interior/BP_Ship_Systems_Widget` (`self.CurrentMenu`)))
  (bind (_hpcurrent _hpmax _magcurrent _magmax _thrustcurrent _thrustmax _m) (`WidgetShipSystems.ReturnWidgetValues` _asbp_ship_systems_widget))
  (set `self.HPCurrent` _hpcurrent)
  (set `self.HpMax` _hpmax)
  (set `self.MagCurrent` _magcurrent)
  (set `self.MagMax` _magmax)
  (set `self.ThrustCurrent` _thrustcurrent)
  (set `self.ThrustMax` _thrustmax)
  (set `self.Money` _m)
  (`self.UpdatePilotHUD`))

(event `LoadFromGame`
  ;[1 1 1] Old Saves
  (bind _returnvalue (`GameplayStatics.DoesSaveGameExist` "TheGame"))
  (if _returnvalue
    (bind _returnvalue_2 (`GameplayStatics.LoadGameFromSlot` "TheGame"))
    (bind _asbp_save_game (cast `/Game/Spacey_BP/BP_SaveGame` _returnvalue_2))
    (set `self.GunLeft` (`/Game/Spacey_BP/BP_SaveGame.PlayerGunLeft` _asbp_save_game))
    (set `self.GunRight` (`/Game/Spacey_BP/BP_SaveGame.PlayerGunRight` _asbp_save_game))
    (set `self.Money` (`/Game/Spacey_BP/BP_SaveGame.Money` _asbp_save_game))
    (set `self.bLoaded` true)))

(fn `ComponentsToSave`
  (returns (Components :type "Array of ActorComponent Object Reference"))
  (return))

(fn `LoadPilot`
  (`|ExecutionSequence`
    (:`then_0`
      (bind _returnvalue (`GameplayStatics.DoesSaveGameExist` "Shared"))
      (if _returnvalue
        (bind _returnvalue_2 (`GameplayStatics.LoadGameFromSlot` "Shared"))
        (bind _asbp_save_game (cast `/Game/Spacey_BP/BP_SaveGame` _returnvalue_2))
        (`|ExecutionSequence`
          (:`then_0`
            (bind (_money _left _right) (`/Game/Spacey_BP/BP_SaveGame.ReturnShared` _asbp_save_game))
            (set `self.Money` _money)
            (set `self.GunLeft` _left)
            (set `self.GunRight` _right))
          (:`then_1`
            (bind (_max _current _drain _regen _bootup _bootupcurrent) (`/Game/Spacey_BP/BP_SaveGame.ReturnShields` _asbp_save_game))
            (set `self.ShieldMax` _max)
            (set `self.ShieldCurrent` _current)
            (set `self.ShieldDrain` _drain)
            (set `self.ShieldRegen` _regen)
            (set `self.ShieldBootUp` _bootup)
            (set `self.ShieldBootUpCurrent` _bootupcurrent))
          (:`then_2`
            (bind (_fire1 _fire2 _power1 _power2) (`/Game/Spacey_BP/BP_SaveGame.ReturnGuns` _asbp_save_game))
            (set `self.Fire1` _fire1)
            (set `self.Fire2` _fire2)
            (set `self.Power1` _power1)
            (set `self.Power2` _power2))
          (:`then_3`
            (bind (_magcurrent _magmax _thrustcurrent _thrustmax) (`/Game/Spacey_BP/BP_SaveGame.ReturnSystems` _asbp_save_game))
            (set `self.MagCurrent` _magcurrent)
            (set `self.MagMax` _magmax)
            (set `self.ThrustCurrent` _thrustcurrent)
            (set `self.ThrustMax` _thrustmax))
          (:`then_4`
            (bind (_location _rotation _healthcurrent _healthmax) (`/Game/Spacey_BP/BP_SaveGame.ReturnBasic` _asbp_save_game))
            (`|ExecutionSequence`
              (:`then_0`
                (if (!= _healthcurrent 0.0)
                  (set `self.HPCurrent` _healthcurrent)))
              (:`then_1`
                (if (!= _healthmax 0.0)
                  (set `self.HpMax` _healthmax))))))))))

(fn `SavePilot`
  (bind _returnvalue (`GameplayStatics.CreateSaveGameObject` "/Game/Spacey_BP/BP_SaveGame.BP_SaveGame_C"))
  (`|ExecutionSequence`
    (:`then_0`
      (`/Game/Spacey_BP/BP_SaveGame.SetShared` _returnvalue (`self.Money`) (`self.GunLeft`) (`self.GunRight`))
      (`/Game/Spacey_BP/BP_SaveGame.SetShields` _returnvalue (`self.ShieldMax`) (`self.ShieldCurrent`) (`self.ShieldDrain`) (`self.ShieldRegen`) (`self.ShieldBootUp`) (`self.ShieldBootUpCurrent`))
      (`/Game/Spacey_BP/BP_SaveGame.SetGuns` _returnvalue (`self.Fire1`) (`self.Fire2`) (`self.Power1`) (`self.Power2`))
      (`/Game/Spacey_BP/BP_SaveGame.SetSystems` _returnvalue (`self.MagCurrent`) (`self.MagMax`) (`self.ThrustCurrent`) (`self.ThrustMax`))
      (`/Game/Spacey_BP/BP_SaveGame.SetBasic` :`self` _returnvalue :`HealthCurrent` (`self.HPCurrent`) :`HealthMax` (`self.HpMax`))
      (`GameplayStatics.SaveGameToSlot` _returnvalue "Shared"))))

(fn `UserConstructionScript`)