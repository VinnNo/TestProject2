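; BP_MenuShip is the main menu ship, flying as animated backdrop while driving menu music and input.
; On BeginPlay it creates default settings if no save exists and spawns WBP_MainMenu.
; A randomly timed loop spawns and destroys a BP_HomingActor as the projectile movement's homing target, toggling child guns' firing after each destroy.
; Up, Down, Accept and Back inputs route to main or settings widgets, with Back restoring the main menu.
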(event `self.ReceiveBeginPlay`
  (`self.SetDefaultSettings`)
  (bind _returnvalue (`GameplayStatics.SpawnSoundAttached` "/Game/Spacey/Audio/Music/Music_Menu.Music_Menu" (`self.RootComponent`) "None" (0.0 0.0 0.0) (struct) "KeepRelativeOffset" false 1.0 1.0 0.0 null null))
  (`AudioComponent.Play` _returnvalue 1.7)
  (`ActorComponent.SetActive` (`self.ParticleSystem1`) false false)
  (`ActorComponent.SetActive` (`self.ParticleSystem`) false false)
  (`self.SpawnMenu`)
  (`KismetSystemLibrary.Delay` (`self.RandomizeFloat` (`self.RandomTime`)))
  (`self.SetFire` true)
  (`self.SpawnHomingActor`)
  (`ActorComponent.SetActive` (`self.ParticleSystem1`) true false)
  (`ActorComponent.SetActive` (`self.ParticleSystem`) true false))

(event `SpawnHomingActor`
  (set `ProjectileMovementComponent.bIsHomingProjectile` true (`self.ProjectileMovement`))
  (bind _returnvalue (`|SpawnActorFromClass` "/Game/Spacey_BP/Player/BP_HomingActor.BP_HomingActor_C" (`KismetMathLibrary.MakeTransform` (`StaticsLibrary.RandomizeVector` (500.0 500.0 0.0))) "Undefined" "OverrideRootScale" null null))
  (bind _output_get (set `self.HomingActor` _returnvalue))
  (set `ProjectileMovementComponent.HomingTargetComponent` (`Actor.RootComponent` _output_get) (`self.ProjectileMovement`))
  (`KismetSystemLibrary.Delay` (`self.RandomizeFloat` (`self.RandomTime`)))
  (`self.DestroyHomingActor`))

(event `SpawnMenu`
  (bind _returnvalue (`|CreateWidget` "/Game/Spacey_BP/UI/WBP_MainMenu.WBP_MainMenu_C" (`GameplayStatics.GetPlayerController` 0)))
  (bind _output_get (set `self.Menu` _returnvalue))
  (`UserWidget.AddToViewport` _output_get 0))

(event `DestroyHomingActor`
  (`self.K2_DestroyActor` (`self.HomingActor`))
  (set `self.HomingActor` null)
  (set `ProjectileMovementComponent.HomingTargetComponent` null (`self.ProjectileMovement`))
  (if (`self.Firing`)
    (set `self.Firing` false)
    (else
      (set `self.Firing` true)))
  (`self.SetFire` (`self.Firing`))
  (`KismetSystemLibrary.Delay` (`self.RandomizeFloat` (`self.RandomTime`)))
  (`self.SpawnHomingActor`))

(event `InputAction|MenuDown` :consume false
  (params (Key :type "Key Structure"))
  (bind _menu (`self.Menu`))
  (:`Pressed`
    (`/Engine/EditorBlueprintResources/StandardMacros.IsValid` _menu
      (:`Is Valid`
        (`/Game/Spacey_BP/UI/WBP_MainMenu.SwitchMenuItem` (`self.Menu`) (+ (`/Game/Spacey_BP/UI/WBP_MainMenu.MenuItem` _menu) 1)))
      (:`Is Not Valid`
        (`self.SettingsUpdate`)))))

(event `InputAction|MenuUp` :consume false
  (params (Key :type "Key Structure"))
  (bind _menu (`self.Menu`))
  (:`Pressed`
    (`/Engine/EditorBlueprintResources/StandardMacros.IsValid` _menu
      (:`Is Valid`
        (`/Game/Spacey_BP/UI/WBP_MainMenu.SwitchMenuItem` (`self.Menu`) (- (`/Game/Spacey_BP/UI/WBP_MainMenu.MenuItem` _menu) 1)))
      (:`Is Not Valid`
        (`self.SettingsUpdate`)))))

(event `SettingsUpdate`
  (`/Engine/EditorBlueprintResources/StandardMacros.IsValid` (`self.SettingMenu`)
    (:`Is Valid`
      (`/Game/Spacey_BP/UI/WBP_ControllerLayout.SwitchMenuItem` (`self.SettingMenu`)))))

(event `InputAction|Accept`
  (params (Key :type "Key Structure"))
  (bind _settingmenu (`self.SettingMenu`))
  (bind _menu (`self.Menu`))
  (:`Pressed`
    (`/Engine/EditorBlueprintResources/StandardMacros.IsValid` _menu
      (:`Is Valid`
        (`/Game/Spacey_BP/UI/WBP_MainMenu.Yes` _menu))
      (:`Is Not Valid`
        (`/Engine/EditorBlueprintResources/StandardMacros.IsValid` _settingmenu
          (:`Is Valid`
            (`/Game/Spacey_BP/UI/WBP_ControllerLayout.Yes` _settingmenu)))))))

(event `InputAction|Back`
  (params (Key :type "Key Structure"))
  (bind _settingmenu (`self.SettingMenu`))
  (:`Pressed`
    (`/Engine/EditorBlueprintResources/StandardMacros.IsValid` _settingmenu
      (:`Is Valid`
        (`Widget.RemoveFromParent` _settingmenu)
        (set `self.SettingMenu` null)
        (if (not (`KismetSystemLibrary.IsValid` (`self.Menu`)))
          (bind _returnvalue (`|CreateWidget` "/Game/Spacey_BP/UI/WBP_MainMenu.WBP_MainMenu_C" (`GameplayStatics.GetPlayerController` 0)))
          (bind _output_get (set `self.Menu` _returnvalue))
          (`UserWidget.AddToViewport` _output_get 0)
          (`GameplayStatics.PlaySound2D` "/Game/Spacey/Audio/SFX/Menus/Widets/minimize_006.minimize_006" 1.0 1.0 0.0 null null))))))

(fn `RandomizeFloat`
  (params (InFloat :type "Float (double-precision)"))
  (returns (OutFloat :type "Float (double-precision)"))
  (return (`KismetMathLibrary.RandomFloatInRange` 0.0 InFloat)))

(fn `SetDefaultSettings`
  (bind _returnvalue (`GameplayStatics.DoesSaveGameExist` "Settings"))
  (if (not _returnvalue)
    (bind _returnvalue_2 (`GameplayStatics.CreateSaveGameObject` "/Game/Spacey_BP/BP_SaveGame.BP_SaveGame_C"))
    (`/Game/Spacey_BP/BP_SaveGame.SetSettings` _returnvalue_2 1 true 1.0 1.0 1.0)
    (`GameplayStatics.SaveGameToSlot` _returnvalue_2 "Settings")))

(fn `SetFire`
  (params (`SetFiring?` :type Boolean))
  (for _array_element (`self.GetAllChildActors` true)
    (bind _asbp_ship_gun_parent (cast `/Game/Spacey_BP/Player/BP_ShipGunParent` _array_element))
    (set `/Game/Spacey_BP/Player/BP_ShipGunParent.bIsFiring` `SetFiring?` _asbp_ship_gun_parent)
    (`/Game/Spacey_BP/Player/BP_ShipGunParent.FireEvent` _asbp_ship_gun_parent)))

(fn `UserConstructionScript`)