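; Player ship pawn, apparently a work-in-progress, with thrust input and experimental turning logic.
; The Thruster axis adds movement input along the ship's forward vector.
; TurnUp and TurnRight axes build a TargetVector, but FindTargetRotation only prints it.
; Yaw turning through RotatingMovement and a roll-and-yaw UpdateRotation event exist but have no live callers here; hit, overlap and debug input just print.
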(event `StopTurn`
  (set `RotatingMovementComponent.RotationRate` (struct) (`self.RotatingMovement`)))

(event `self.ReceiveTick`
  (params (DeltaSeconds :type "Float (single-precision)")))

(event `self.StaticMesh.OnComponentHit`
  (params (HitComponent :type "PrimitiveComponent Object Reference") (OtherActor :type "Actor Object Reference") (OtherComp :type "PrimitiveComponent Object Reference") (NormalImpulse :type "Vector Structure") (Hit :type "HitResult Structure (by ref)"))
  (`KismetSystemLibrary.PrintString` "Hit"))

(event `InputAxis|MoveRight`
  (params (AxisValue :type "Float (single-precision)")))

(event `InputAxis|Thruster`
  (params (AxisValue :type "Float (single-precision)"))
  (`self.AddMovementInput` (`self.GetActorForwardVector`) AxisValue))

(event `Turn`
  (bind (_rotationrate_roll _rotationrate_pitch _rotationrate_yaw) (`KismetMathLibrary.BreakRotator` (`RotatingMovementComponent.RotationRate` (`self.RotatingMovement`))))
  (set `self.CurrentTurnRate` _rotationrate_yaw)
  (`|ExecutionSequence`
    (:`then_0`
      (if (> (`self.GetInputAxisValue`) 0.0)
        (if (< (`self.CurrentTurnRate`) (`self.TurnSpeed`))
          (set `self.CurrentTurnRate` (+ (`GameplayStatics.GetWorldDeltaSeconds`) (`self.TurnSpeed`))))
        (elif (> (`self.CurrentTurnRate`) (- 0.0 (`self.TurnSpeed`)))
          (set `self.CurrentTurnRate` (- (`GameplayStatics.GetWorldDeltaSeconds`) (`self.TurnSpeed`))))))
    (:`then_1`
      (set `RotatingMovementComponent.RotationRate` (`KismetMathLibrary.MakeRotator` 0.0 0.0 (`self.CurrentTurnRate`)) (`self.RotatingMovement`)))))

(event `InputAxis|TurnUp`
  (params (AxisValue :type "Float (single-precision)"))
  (bind (_targetvector_x _targetvector_y) (`KismetMathLibrary.BreakVector` (`self.TargetVector`)))
  (set `self.TargetVector` (`KismetMathLibrary.MakeVector` AxisValue _targetvector_y))
  (`self.FindTargetRotation` :!label _label))

(event `InputAction|Action_Debug`
  (params (Key :type "Key Structure"))
  (:`Pressed`
    (`KismetSystemLibrary.PrintString` (`KismetStringLibrary.Conv_DoubleToString` (`self.CurrentTurnRate`)))))

(event `InputAxis|TurnRight`
  (params (AxisValue :type "Float (single-precision)"))
  (bind _targetvector_x (`KismetMathLibrary.BreakVector` (`self.TargetVector`)))
  (set `self.TargetVector` (`KismetMathLibrary.MakeVector` _targetvector_x AxisValue))
  (goto _label))

(event `self.StaticMesh.OnComponentBeginOverlap`
  (params (OverlappedComponent :type "PrimitiveComponent Object Reference") (OtherActor :type "Actor Object Reference") (OtherComp :type "PrimitiveComponent Object Reference") (OtherBodyIndex :type Integer) (bFromSweep :type Boolean) (SweepResult :type "HitResult Structure (by ref)"))
  (`KismetSystemLibrary.PrintString` "Overlap"))

(event `FindTargetRotation`
  (`KismetSystemLibrary.PrintString` (`KismetStringLibrary.Conv_VectorToString` (`self.TargetVector`))))

(event `UpdateRotation`
  (params (Value :type "Float (double-precision)"))
  (bind _returnvalue_roll (`KismetMathLibrary.BreakRotator` (`self.K2_GetActorRotation`)))
  (if (> Value 0.0)
    (`self.K2_SetActorRotation` (`KismetMathLibrary.MakeRotator` (* Value (+ _returnvalue_roll (`self.RollSpeed`))) 0.0 (* Value (`self.TurnSpeed`))))))

(fn `UserConstructionScript`)