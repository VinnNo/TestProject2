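; BP_Player_EndGame is the player Blueprint for the game-won screen, handling its display and the exit to the main menu.
; BeginPlay clears existing widgets and adds WBP_GameWon to the viewport.
; The Restart event and the Accept and Back inputs share one path: create a BP_SaveGame object, call ClearAll on it, remove all widgets and open Map_Menu.
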(event `self.ReceiveBeginPlay`
  (`WidgetLayoutLibrary.RemoveAllWidgets`)
  (bind _returnvalue (`|CreateWidget` "/Game/Spacey_BP/UI/WBP_GameWon.WBP_GameWon_C" (`GameplayStatics.GetPlayerController` 0)))
  (bind _output_get (set `self.Menu` _returnvalue))
  (`UserWidget.AddToViewport` _output_get 0))

(event `Restart`
  (bind _returnvalue (`GameplayStatics.CreateSaveGameObject` "/Game/Spacey_BP/BP_SaveGame.BP_SaveGame_C" :!label _label))
  (`/Game/Spacey_BP/BP_SaveGame.ClearAll` _returnvalue)
  (`WidgetLayoutLibrary.RemoveAllWidgets`)
  (`GameplayStatics.OpenLevel` "Map_Menu"))

(event `InputAction|Accept`
  (params (Key :type "Key Structure"))
  (:`Pressed`
    (goto _label)))

(event `InputAction|Back`
  (params (Key :type "Key Structure"))
  (:`Pressed`
    (goto _label)))

(fn `UserConstructionScript`)