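; Parent Blueprint for gem pickups that add money to the player ship, randomized on spawn and destroyed when their lifetime ends.
; After a short delay, the OnRandomized event applies random value, scale, mesh and material.
; The Sight component sets or clears the player-found state and target as the ship's mesh enters or leaves.
; Gem mesh overlap with that same ship component awards the value and destroys the pickup.
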(event `self.ReceiveBeginPlay`
  (`self.RandomizeAll`)
  (`self.SetRotation`)
  (`KismetSystemLibrary.Delay` (`self.LifeTime`))
  (`self.K2_DestroyActor`))

(event `self.OnRandomized`
  (bind _gemmesh (`self.GemMesh`))
  (`KismetSystemLibrary.Delay` 0.1)
  (set `self.BaseValue` (+ (`self.BaseValue`) (`self.RandomValue`)))
  (`self.SetActorScale3D` (+ (`self.RandomScale`) (`self.GetActorScale3D`)))
  (`StaticMeshComponent.SetStaticMesh` _gemmesh (`self.RandomMesh`))
  (`PrimitiveComponent.SetMaterial` _gemmesh 0 (`self.RandomMaterial`)))

(event `self.Sight.OnComponentBeginOverlap`
  (params (OverlappedComponent :type "PrimitiveComponent Object Reference") (OtherActor :type "Actor Object Reference") (OtherComp :type "PrimitiveComponent Object Reference") (OtherBodyIndex :type Integer) (bFromSweep :type Boolean) (SweepResult :type "HitResult Structure (by ref)"))
  (`self.SightEntered` OtherActor OtherComp))

(event `SightEntered`
  (params (Actor :type "Actor Object Reference") (Comp :type "PrimitiveComponent Object Reference"))
  (bind _asbp_player_ship (cast `/Game/Spacey_BP/Player/BP_PlayerShip` Actor))
  (if (== Comp (`PlayerShipBase.ShipMeshComponent` _asbp_player_ship))
    (`self.SetPlayerFound` true)
    (set `self.TargetActor` _asbp_player_ship)))

(event `SightLeft`
  (params (Actor :type "Actor Object Reference") (Comp :type "PrimitiveComponent Object Reference"))
  (bind _asbp_player_ship (cast `/Game/Spacey_BP/Player/BP_PlayerShip` Actor))
  (if (== Comp (`PlayerShipBase.ShipMeshComponent` _asbp_player_ship))
    (`self.SetPlayerFound` false)
    (set `self.TargetActor` null)))

(event `self.Sight.OnComponentEndOverlap`
  (params (OverlappedComponent :type "PrimitiveComponent Object Reference") (OtherActor :type "Actor Object Reference") (OtherComp :type "PrimitiveComponent Object Reference") (OtherBodyIndex :type Integer))
  (`self.SightLeft` OtherActor OtherComp))

(event `OverlapPlayer`
  (params (Actor :type "Actor Object Reference") (Comp :type "PrimitiveComponent Object Reference"))
  (bind _asbp_player_ship (cast `/Game/Spacey_BP/Player/BP_PlayerShip` Actor))
  (if (== Comp (`PlayerShipBase.ShipMeshComponent` _asbp_player_ship))
    (`/Game/Spacey_BP/Player/BP_PlayerShip.UpdateMoney` _asbp_player_ship (`self.BaseValue`))
    (`self.K2_DestroyActor`)))

(event `self.GemMesh.OnComponentBeginOverlap`
  (params (OverlappedComponent :type "PrimitiveComponent Object Reference") (OtherActor :type "Actor Object Reference") (OtherComp :type "PrimitiveComponent Object Reference") (OtherBodyIndex :type Integer) (bFromSweep :type Boolean) (SweepResult :type "HitResult Structure (by ref)"))
  (`self.OverlapPlayer` OtherActor OtherComp))

(fn `UserConstructionScript`)