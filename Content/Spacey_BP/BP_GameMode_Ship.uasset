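; Game mode for a wave-based spaceship shooter, handling wave feedback, boss spawning and saved wave progress.
; Wave, timer and debounced enemy-death events drive the player ship's wave HUD, banners, sounds, final countdown and mobile-only start button.
; Wave end shows a health-scaled bonus, flags boss wave 20, and opens the end-game map at wave 21.
; DoBossWave spawns the boss, then recursively adds enemies on a delay until the player dies.
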(event `SpawnStartWaveButton`
  (bind _asbp_player_ship (cast `/Game/Spacey_BP/Player/BP_PlayerShip` (`GameplayStatics.GetPlayerPawn` 0)))
  (if (and (`PlayerShipBase.bIsMobile` _asbp_player_ship) (not (`self.bWaveActive`)))
    (bind _returnvalue (`|CreateWidget` "/Game/Spacey_BP/UI/WBP_Wave_Start-End.WBP_Wave_Start-End_C" (`GameplayStatics.GetPlayerController` 0)))
    (bind _output_get (set `self.StartWaveButton` _returnvalue))
    (`UserWidget.AddToViewport` _output_get 0)))

(event `DestroyStartWaveButton`
  (bind _startwavebutton (`self.StartWaveButton`))
  (`/Engine/EditorBlueprintResources/StandardMacros.IsValid` _startwavebutton
    (:`Is Valid`
      (`Widget.RemoveFromParent` _startwavebutton)
      (set `self.StartWaveButton` null))))

(event `self.ReceiveBeginPlay`
  (`self.LoadGameMode`)
  (`self.SpawnStartWaveButton`))

(event `EnemyShipDeath`
  (`KismetSystemLibrary.RetriggerableDelay` 0.05)
  (`self.UpdateEnemyShipCount`)
  (bind _asbp_player_ship (cast `/Game/Spacey_BP/Player/BP_PlayerShip` (`GameplayStatics.GetPlayerPawn` 0)))
  (bind _widgetwaves (`/Game/Spacey_BP/Player/BP_PlayerShip.WidgetWaves` _asbp_player_ship))
  (`/Engine/EditorBlueprintResources/StandardMacros.IsValid` _widgetwaves
    (:`Is Valid`
      (`WidgetWaveDisplay.UpdateWidgetValues` _widgetwaves (`self.WaveCurrent`) (`self.TimeMinutes`) (`self.TimeSeconds`) (`self.EnemyCount`) (`self.bWaveActive`)))))

(event `self.OnTimeUpdated`
  (`|ExecutionSequence`
    (:`then_0`
      (bind _asbp_player_ship (cast `/Game/Spacey_BP/Player/BP_PlayerShip` (`GameplayStatics.GetPlayerPawn` 0)))
      (bind _widgetwaves (`/Game/Spacey_BP/Player/BP_PlayerShip.WidgetWaves` _asbp_player_ship))
      (`/Engine/EditorBlueprintResources/StandardMacros.IsValid` _widgetwaves
        (:`Is Valid`
          (`WidgetWaveDisplay.UpdateWidgetValues` _widgetwaves (`self.WaveCurrent`) (`self.TimeMinutes`) (`self.TimeSeconds`) (`self.EnemyCount`) (`self.bWaveActive`)))))
    (:`then_1`
      (if (and (== (`self.TimeMinutes`) 0) (<= (`self.TimeSeconds`) 5) (!= (`self.TimeSeconds`) 0))
        (set `self.bCanGoInside` false)
        (`self.SpawnFinalCountDown`)))))

(event `self.OnWaveStarted`
  (`self.SpawnWaveStart-End` true)
  (`|ExecutionSequence`
    (:`then_0`
      (`KismetSystemLibrary.Delay` 0.1)
      (bind _asbp_player_ship (cast `/Game/Spacey_BP/Player/BP_PlayerShip` (`GameplayStatics.GetPlayerPawn` 0)))
      (bind _widgetwaves (`/Game/Spacey_BP/Player/BP_PlayerShip.WidgetWaves` _asbp_player_ship))
      (`/Engine/EditorBlueprintResources/StandardMacros.IsValid` _widgetwaves
        (:`Is Valid`
          (`WidgetWaveDisplay.UpdateWidgetValues` _widgetwaves (`self.WaveCurrent`) (`self.TimeMinutes`) (`self.TimeSeconds`) (`self.EnemyCount`) (`self.bWaveActive`))
          (`GameplayStatics.PlaySoundAtLocation` "/Game/Spacey/Audio/SFX/Menus/In-Game/zapThreeToneDown.zapThreeToneDown" (`self.K2_GetActorLocation` _asbp_player_ship) (struct) 1.0 1.0 0.0 null null null)
          (set `self.bCanGoInside` false))))
    (:`then_1`
      (if (== (`self.WaveCurrent`) 20)
        (`KismetSystemLibrary.Delay` 0.2)
        (bind _returnvalue (`|CreateWidget` "/Game/Spacey_BP/UI/Ship_Exterior/WBP_BossWaveReadout.WBP_BossWaveReadout_C" (`GameplayStatics.GetPlayerController` 0)))
        (`UserWidget.AddToViewport` _returnvalue 0)))
    (:`then_2`
      (`self.DestroyStartWaveButton`))))

(event `SpawnFinalCountDown`
  (`|ExecutionSequence`
    (:`then_0`
      (bind _returnvalue (`|CreateWidget` "/Game/Spacey_BP/UI/WBP_FinalCountDown.WBP_FinalCountDown_C" (`GameplayStatics.GetPlayerController` 0)))
      (`/Game/Spacey_BP/UI/WBP_FinalCountDown.SetValue` _returnvalue (`self.TimeSeconds`))
      (`UserWidget.AddToViewport` _returnvalue 0))
    (:`then_1`
      (`self.DestroyStartWaveButton`))))

(event `self.OnWaveEnded`
  (`self.SpawnWaveStart-End` false)
  (if (!= (`self.WaveCurrent`) 21)
    (`|ExecutionSequence`
      (:`then_0`
        (`|ExecutionSequence`
          (:`then_0`
            (`KismetSystemLibrary.Delay` 0.1)
            (bind _asbp_player_ship (cast `/Game/Spacey_BP/Player/BP_PlayerShip` (`GameplayStatics.GetPlayerPawn` 0)))
            (bind _widgetwaves (`/Game/Spacey_BP/Player/BP_PlayerShip.WidgetWaves` _asbp_player_ship))
            (`/Engine/EditorBlueprintResources/StandardMacros.IsValid` _widgetwaves
              (:`Is Valid`
                (`WidgetWaveDisplay.UpdateWidgetValues` _widgetwaves (`self.WaveCurrent`) (`self.TimeMinutes`) (`self.TimeSeconds`) (`self.EnemyCount`) (`self.bWaveActive`))
                (`GameplayStatics.PlaySoundAtLocation` "/Game/Spacey/Audio/SFX/Menus/In-Game/zapThreeToneUp.zapThreeToneUp" (`self.K2_GetActorLocation` _asbp_player_ship) (struct) 1.0 1.0 0.0 null null null))))
          (:`then_1`
            (bind _asbp_player_ship_2 (cast `/Game/Spacey_BP/Player/BP_PlayerShip` (`GameplayStatics.GetPlayerPawn` 0)))
            (bind _returnvalue (`|CreateWidget` "/Game/Spacey_BP/UI/Ship_Exterior/WBP_WaveBonus.WBP_WaveBonus_C" (`GameplayStatics.GetPlayerController` 0)))
            (`/Game/Spacey_BP/UI/Ship_Exterior/WBP_WaveBonus.SetBonusAmount` _returnvalue (`KismetMathLibrary.FTrunc` (* (`self.WaveCurrent`) (* (`HealthComponent.GetHealthAsPercent` (`/Game/Spacey_BP/Player/BP_PlayerShip.Health` _asbp_player_ship_2)) 1500.0))))
            (`UserWidget.AddToViewport` _returnvalue 0))))
      (:`then_1`
        (if (== (`self.WaveCurrent`) 20)
          (`KismetSystemLibrary.Delay` 0.2)
          (bind _returnvalue_2 (`|CreateWidget` "/Game/Spacey_BP/UI/Ship_Exterior/WBP_BossWaveReadout.WBP_BossWaveReadout_C" (`GameplayStatics.GetPlayerController` 0)))
          (`UserWidget.AddToViewport` _returnvalue_2 0)))
      (:`then_2`
        (`self.SpawnStartWaveButton`)))
    (else
      (`GameplayStatics.OpenLevel` "Map_EndGame"))))

(event `SpawnWaveStart-End`
  (params (`bStarted?` :type Boolean))
  (bind _returnvalue (`|CreateWidget` "/Game/Spacey_BP/UI/WBP_Wave_StartEnd.WBP_Wave_StartEnd_C" (`GameplayStatics.GetPlayerController` 0)))
  (`|ExecutionSequence`
    (:`then_0`
      (if `bStarted?`
        (`/Game/Spacey_BP/UI/WBP_Wave_StartEnd.SetValue` _returnvalue "Wave Start!")
        (else
          (`/Game/Spacey_BP/UI/WBP_Wave_StartEnd.SetValue` _returnvalue "Wave Ended!"))))
    (:`then_1`
      (`UserWidget.AddToViewport` _returnvalue 0))))

(event `self.DoBossWave`
  (`|SpawnActorFromClass` "/Game/Spacey_BP/Enemies/BP_BossShip1.BP_BossShip1_C" (`KismetMathLibrary.MakeTransform` (-500.0 2065.0 700.0)) "AdjustIfPossibleButAlwaysSpawn" "OverrideRootScale" null null)
  (`KismetSystemLibrary.Delay` 5.0)
  (`self.SpawnBossWaveEnemies`))

(event `SpawnBossWaveEnemies`
  (bind (_spawnrange_x _spawnrange_y _spawnrange_z) (`KismetMathLibrary.BreakVector` (`self.SpawnRange`)))
  (bind (_outvector_x _outvector_y) (`KismetMathLibrary.BreakVector` (`StaticsLibrary.RandomizeVector` (`self.SpawnRange`))))
  (if (not (`self.bPlayerDead`))
    (`|SpawnActorFromClass` "/Game/Spacey_BP/Enemies/BP_EnemyShip1.BP_EnemyShip1_C" (`KismetMathLibrary.MakeTransform` (`KismetMathLibrary.MakeVector` _outvector_x _outvector_y _spawnrange_z)) "AdjustIfPossibleButAlwaysSpawn" "OverrideRootScale" null null)
    (`KismetSystemLibrary.Delay` 10.0)
    (`self.SpawnBossWaveEnemies`)))

(fn `LoadGameMode`
  (bind _returnvalue (`GameplayStatics.DoesSaveGameExist` "GameMode"))
  (if _returnvalue
    (bind _returnvalue_2 (`GameplayStatics.LoadGameFromSlot` "GameMode"))
    (bind _asbp_save_game (cast `/Game/Spacey_BP/BP_SaveGame` _returnvalue_2))
    (bind (_active _time _wave _1 _2 _3 _4 _idletime) (`/Game/Spacey_BP/BP_SaveGame.ReturnGameMode` _asbp_save_game))
    (set `self.bWaveActive` _active)
    (set `self.WaveUpTimeCurrent` _time)
    (set `self.WaveCurrent` _wave)
    (set `self.Type1Count` _1)
    (set `self.Type2Count` _2)
    (set `self.Type3Count` _3)
    (set `self.Type4Count` _4)
    (set `self.StartingIdleTime` _idletime)))

(fn `SaveGameMode`
  (bind _returnvalue (`GameplayStatics.CreateSaveGameObject` "/Game/Spacey_BP/BP_SaveGame.BP_SaveGame_C"))
  (`/Game/Spacey_BP/BP_SaveGame.SetGameMode` _returnvalue (`self.bWaveActive`) (`self.WaveUpTimeCurrent`) (`self.WaveCurrent`) (`self.Type1Count`) (`self.Type2Count`) (`self.Type3Count`) (`self.Type4Count`) (`self.StartingIdleTime`))
  (`GameplayStatics.SaveGameToSlot` _returnvalue "GameMode"))

(fn `UserConstructionScript`)