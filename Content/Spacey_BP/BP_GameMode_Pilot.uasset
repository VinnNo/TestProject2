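; Game mode for the pilot segment, which runs against the wave timer and returns the player to Map_2.
; BeginPlay restores wave state from the "GameMode" save slot; SaveGameMode writes it back but is not called here.
; OnTimeUpdated refreshes the pilot's wave display with enemy readouts hidden, then at five seconds left calls RetrieveAll and loads the map.
; Other wave, boss and death events are empty, leaving their ship-combat logic disconnected.
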(event `self.ReceiveBeginPlay`
  (`self.LoadGameMode`))

(event `EnemyShipDeath`)

(event `self.OnTimeUpdated`
  (if (or (> (`self.TimeSeconds`) 5) (> (`self.TimeMinutes`) 0))
    (bind _asbp_pilot (cast `/Game/Spacey_BP/Player/BP_Pilot` (`GameplayStatics.GetPlayerPawn` 0)))
    (bind _wavedisplay (`/Game/Spacey_BP/Player/BP_Pilot.WaveDisplay` _asbp_pilot))
    (`/Engine/EditorBlueprintResources/StandardMacros.IsValid` _wavedisplay
      (:`Is Valid`
        (`WidgetWaveDisplay.UpdateWidgetValues` _wavedisplay (`self.WaveCurrent`) (`self.TimeMinutes`) (`self.TimeSeconds`) (`self.EnemyCount`) (`self.bWaveActive`))
        (`Widget.SetVisibility` (`WidgetWaveDisplay.EnemyCountLabel` _wavedisplay) "Hidden")
        (`Widget.SetVisibility` (`/Game/Spacey_BP/UI/WBP_WaveDisplayPilot.EnemyReadoutLabel` _wavedisplay) "Hidden")))
    (else
      (bind _asbp_pilot_2 (cast `/Game/Spacey_BP/Player/BP_Pilot` (`GameplayStatics.GetPlayerPawn` 0)))
      (`/Game/Spacey_BP/Player/BP_Pilot.RetrieveAll` _asbp_pilot_2)
      (`KismetSystemLibrary.Delay` 0.2)
      (`GameplayStatics.OpenLevel` "Map_2"))))

(event `self.OnWaveStarted`)

(event `self.OnWaveEnded`)

(event `self.DoBossWave`)

(event `SpawnBossWaveEnemies`)

(fn `LoadGameMode`
  (bind _returnvalue (`GameplayStatics.DoesSaveGameExist` "GameMode"))
  (if _returnvalue
    (bind _returnvalue_2 (`GameplayStatics.LoadGameFromSlot` "GameMode"))
    (bind _asbp_save_game (cast `/Game/Spacey_BP/BP_SaveGame` _returnvalue_2))
    (bind (_active _time _wave _1 _2 _3 _4 _idletime) (`/Game/Spacey_BP/BP_SaveGame.ReturnGameMode` _asbp_save_game))
    (set `self.bWaveActive` _active)
    (set `self.WaveUpTimeCurrent` _time)
    (set `self.WaveCurrent` _wave)
    (set `self.Type1Count` _1)
    (set `self.Type2Count` _2)
    (set `self.Type3Count` _3)
    (set `self.Type4Count` _4)
    (set `self.StartingIdleTime` _idletime)))

(fn `SaveGameMode`
  (bind _returnvalue (`GameplayStatics.CreateSaveGameObject` "/Game/Spacey_BP/BP_SaveGame.BP_SaveGame_C"))
  (`/Game/Spacey_BP/BP_SaveGame.SetGameMode` _returnvalue (`self.bWaveActive`) (`self.WaveUpTimeCurrent`) (`self.WaveCurrent`) (`self.Type1Count`) (`self.Type2Count`) (`self.Type3Count`) (`self.Type4Count`) (`self.StartingIdleTime`))
  (`GameplayStatics.SaveGameToSlot` _returnvalue "GameMode"))

(fn `UserConstructionScript`)